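; First-person hands pawn that previews the S96 sniper rifle animation set through number-key presses.
; Equip spawns BP_SR_S96_P once, attaches it to the hand socket and disables the weapon's input.
; Each key plays a hands animation directly, with fixed Delays chaining follow-ups such as bolt chambering or returning to idle.
; Reload and shoot also call the rifle's matching functions, finding it via GetAllActorsOfClass rather than a stored reference.
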(event EventBeginPlay
  ;[1 1 1] Player Input
  (Input|EnableInput (Game|GetPlayerController 0)))

(event Input|KeyboardEvents|4
  (params (Key :type Key%20Structure))
  ;[1 1 1] Shooting
  (:Pressed
    (if (Variables|Default|GetWeapon%20is%20Spawned)
      (bind _outactors (Actor|GetAllActorsOfClass "/Game/FPS/Weapons/Sniper/SR_S96/Blueprints/BP_SR_S96_P.BP_SR_S96_P_C"))
      (Default|HandsSooting (Utilities|Array|Get(acopy) _outactors)))
    (Components|Animation|PlayAnimation (Variables|Default|GetHands) "/Game/FPS/Weapons/Sniper/SR_S96/Animations/FPS_Hands_Animations/AS_Hands_SR_S96_Shooting.AS_Hands_SR_S96_Shooting" false)
    (Utilities|FlowControl|Delay 0.5)
    (Components|Animation|PlayAnimation (Variables|Default|GetHands) "/Game/FPS/Weapons/Sniper/SR_S96/Animations/FPS_Hands_Animations/AS_Hands_SR_S96_Bolt_Chamber.AS_Hands_SR_S96_Bolt_Chamber" false)
    (Utilities|FlowControl|Delay 1.467)
    (Components|Animation|PlayAnimation (Variables|Default|GetHands) "/Game/FPS/Weapons/Sniper/SR_S96/Animations/FPS_Hands_Animations/AS_Hands_SR_S96_Idle_Standing.AS_Hands_SR_S96_Idle_Standing" true)))

(event Input|KeyboardEvents|0
  (params (Key :type Key%20Structure))
  ;[1 1 1] Weapon unequip
  (:Pressed
    (Components|Animation|PlayAnimation (Variables|Default|GetHands) "/Game/FPS/Weapons/Sniper/SR_S96/Animations/FPS_Hands_Animations/AS_Hands_SR_S96_UnEquip.AS_Hands_SR_S96_UnEquip" false)))

(event Input|KeyboardEvents|6
  (params (Key :type Key%20Structure))
  (bind _hands (Variables|Default|GetHands))
  ;[1 1 1] Weapon Inspect
  (:Pressed
    (Components|Animation|PlayAnimation _hands "/Game/FPS/Weapons/Sniper/SR_S96/Animations/FPS_Hands_Animations/AS_Hands_SR_S96_WeaponInspect.AS_Hands_SR_S96_WeaponInspect" false)
    (Utilities|FlowControl|Delay 5.667)
    (Components|Animation|PlayAnimation _hands "/Game/FPS/Weapons/Sniper/SR_S96/Animations/FPS_Hands_Animations/AS_Hands_SR_S96_Idle_Standing.AS_Hands_SR_S96_Idle_Standing" true)))

(event Input|KeyboardEvents|7
  (params (Key :type Key%20Structure))
  ;[1 1 1] Scope Aim
  (:Pressed
    (Components|Animation|PlayAnimation (Variables|Default|GetHands) "/Game/FPS/Weapons/Sniper/SR_S96/Animations/FPS_Hands_Animations/AS_Hands_SR_S96_Aim_Scope.AS_Hands_SR_S96_Aim_Scope" false)))

(event Input|KeyboardEvents|9
  (params (Key :type Key%20Structure))
  (bind _hands (Variables|Default|GetHands))
  ;[1 1 1] Scope UnAim
  (:Pressed
    (Components|Animation|PlayAnimation _hands "/Game/FPS/Weapons/Sniper/SR_S96/Animations/FPS_Hands_Animations/AS_Hands_SR_S96_UnAim.AS_Hands_SR_S96_UnAim" false)
    (Utilities|FlowControl|Delay 0.427)
    (Components|Animation|PlayAnimation _hands "/Game/FPS/Weapons/Sniper/SR_S96/Animations/FPS_Hands_Animations/AS_Hands_SR_S96_Idle_Standing.AS_Hands_SR_S96_Idle_Standing" true)))

(event Input|KeyboardEvents|8
  (params (Key :type Key%20Structure))
  ;[1 1 1] Aim Shooting
  (:Pressed
    (if (Variables|Default|GetWeapon%20is%20Spawned)
      (bind _outactors (Actor|GetAllActorsOfClass "/Game/FPS/Weapons/Sniper/SR_S96/Blueprints/BP_SR_S96_P.BP_SR_S96_P_C"))
      (Default|HandsSooting (Utilities|Array|Get(acopy) _outactors)))
    (Components|Animation|PlayAnimation (Variables|Default|GetHands) "/Game/FPS/Weapons/Sniper/SR_S96/Animations/FPS_Hands_Animations/AS_Hands_SR_S96_Aim_Shoot.AS_Hands_SR_S96_Aim_Shoot" false)
    (Utilities|FlowControl|Delay 0.5)
    (Components|Animation|PlayAnimation (Variables|Default|GetHands) "/Game/FPS/Weapons/Sniper/SR_S96/Animations/FPS_Hands_Animations/AS_Hands_SR_S96_Aimed_Bolt_Chamber.AS_Hands_SR_S96_Aimed_Bolt_Chamber" false)))

(event Input|KeyboardEvents|3
  (params (Key :type Key%20Structure))
  (bind _hands (Variables|Default|GetHands))
  ;[1 1 1] Running
  (:Pressed
    (Components|Animation|PlayAnimation _hands "/Game/FPS/Weapons/Sniper/SR_S96/Animations/FPS_Hands_Animations/AS_Hands_SR_S96_Running.AS_Hands_SR_S96_Running" true))
  (:Released
    (Components|Animation|PlayAnimation _hands "/Game/FPS/Weapons/Sniper/SR_S96/Animations/FPS_Hands_Animations/AS_Hands_SR_S96_Idle_Standing.AS_Hands_SR_S96_Idle_Standing" true)))

(event Input|KeyboardEvents|1
  (params (Key :type Key%20Structure))
  ;[1 1 1] Weapon Equip
  (:Pressed
    (if (Variables|Default|GetWeapon%20is%20Spawned)
      _
      (else
        (Variables|Default|SetWeapon%20is%20Spawned true)
        (bind _returnvalue (Game|SpawnActorfromClass "/Game/FPS/Weapons/Sniper/SR_S96/Blueprints/BP_SR_S96_P.BP_SR_S96_P_C" (Transformation|GetSocketTransform (Variables|Default|GetHands) "cc_ItemHolder_rSocket" "RTS_World") "DontSpawnIfColliding" 0 0))
        (Transformation|AttachComponentToComponent _returnvalue (Variables|Default|GetHands) "cc_ItemHolder_rSocket" "SnapToTarget" "SnapToTarget" "SnapToTarget" true)
        (bind _outactors (Actor|GetAllActorsOfClass "/Game/FPS/Weapons/Sniper/SR_S96/Blueprints/BP_SR_S96_P.BP_SR_S96_P_C"))
        (Default|DisableInputforWeapon (Utilities|Array|Get(acopy) _outactors))))
    (Components|Animation|PlayAnimation (Variables|Default|GetHands) "/Game/FPS/Weapons/Sniper/SR_S96/Animations/FPS_Hands_Animations/AS_Hands_SR_S96_Equip.AS_Hands_SR_S96_Equip" false)
    (Utilities|FlowControl|Delay 0.8)
    (Components|Animation|PlayAnimation (Variables|Default|GetHands) "/Game/FPS/Weapons/Sniper/SR_S96/Animations/FPS_Hands_Animations/AS_Hands_SR_S96_Idle_Standing.AS_Hands_SR_S96_Idle_Standing" true)))

(event Input|KeyboardEvents|5
  (params (Key :type Key%20Structure))
  ;[1 1 1] Reload
  (:Pressed
    (if (Variables|Default|GetWeapon%20is%20Spawned)
      (bind _outactors (Actor|GetAllActorsOfClass "/Game/FPS/Weapons/Sniper/SR_S96/Blueprints/BP_SR_S96_P.BP_SR_S96_P_C"))
      (Default|HandsReloading (Utilities|Array|Get(acopy) _outactors)))
    (Components|Animation|PlayAnimation (Variables|Default|GetHands) "/Game/FPS/Weapons/Sniper/SR_S96/Animations/FPS_Hands_Animations/AS_Hands_SR_S96_Reload.AS_Hands_SR_S96_Reload" false)
    (Utilities|FlowControl|Delay 2.133)
    (Components|Animation|PlayAnimation (Variables|Default|GetHands) "/Game/FPS/Weapons/Sniper/SR_S96/Animations/FPS_Hands_Animations/AS_Hands_SR_S96_Idle_Standing.AS_Hands_SR_S96_Idle_Standing" true)))

(event Input|KeyboardEvents|2
  (params (Key :type Key%20Structure))
  (bind _hands (Variables|Default|GetHands))
  ;[1 1 1] Walking
  (:Pressed
    (Components|Animation|PlayAnimation _hands "/Game/FPS/Weapons/Sniper/SR_S96/Animations/FPS_Hands_Animations/AS_Hands_SR_S96_Walking.AS_Hands_SR_S96_Walking" true))
  (:Released
    (Components|Animation|PlayAnimation _hands "/Game/FPS/Weapons/Sniper/SR_S96/Animations/FPS_Hands_Animations/AS_Hands_SR_S96_Idle_Standing.AS_Hands_SR_S96_Idle_Standing" true)))

(fn ConstructionScript)