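; BP_SR_S96_P is the S96 sniper rifle weapon Blueprint, playing shoot, bolt and reload animations.
; Keys 1 and 2 or the HandsSooting and HandsReloading events trigger firing and reloading, with an event disabling direct input when hands hold it.
; Firing chambers the bolt after a delay, then spawns, impulses and socket-attaches a shell and activates extractor smoke.
; Reloading briefly hides the magazine ammo mesh.
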(event Custom|Disable%20input%20for%20weapon
  ;[1 1 1] Disabling imput when hands are holding weapon
  (Input|DisableInput 0))

(event Custom|Hands%20Sooting
  (bind _sr_s96_skeletal (Variables|Default|GetSR_S96_Skeletal))
  (bind _returnvalue (Transformation|GetSocketRotation _sr_s96_skeletal "Shell_Socket"))
  (bind _returnvalue_2 (Math|Vector|GetRightVector _returnvalue))
  ;[1 1 1] Single Shoot
  (Components|Animation|PlayAnimation (Variables|Default|GetSR_S96_Skeletal) "/Game/FPS/Weapons/Sniper/SR_S96/Animations/SR_S96_Animations/AS_Weapon_SR_S96_Shoot.AS_Weapon_SR_S96_Shoot" false)
  ;[1 1 1] Bolt Chamber
  (Utilities|FlowControl|Delay 0.5)
  (Components|Animation|PlayAnimation (Variables|Default|GetSR_S96_Skeletal) "/Game/FPS/Weapons/Sniper/SR_S96/Animations/SR_S96_Animations/AS_Weapon_SR_S96_Bolt_Chamber.AS_Weapon_SR_S96_Bolt_Chamber" false)
  (Utilities|FlowControl|Delay 0.6)
  (bind _returnvalue_3 (Game|SpawnActorfromClass "/Game/FPS/Weapons/Sniper/SR_S96/Blueprints/BP_SR_S96_P_Shell.BP_SR_S96_P_Shell_C" (Math|Transform|MakeTransform (Transformation|GetSocketLocation _sr_s96_skeletal "Shell_Socket") _returnvalue "1.000000,1.000000,1.000000") "Undefined" 0 0))
  (Physics|AddImpulse (Variables|/Game/FPS/Weapons/Sniper/SR_S96/Blueprints/BP_SR_S96_P_Shell.BP_SR_S96_P_Shell_C|GetCase _returnvalue_3) (Math|Vector|MakeVector (.x _returnvalue_2) (+ (.y _returnvalue_2) 5e+01) (.z _returnvalue_2)) "Shell_Socket" false)
  (Transformation|AttachComponentToComponent _returnvalue_3 _sr_s96_skeletal "Shell_Socket" "SnapToTarget" "SnapToTarget" "SnapToTarget" true)
  (Components|Activation|Activate (Variables|Default|GetPS_SR_96_P_Extractor_Smoke) false))

(event Custom|Hands%20Reloading
  ;[1 1 1] Reload
  (Components|Animation|PlayAnimation (Variables|Default|GetSR_S96_Skeletal) "/Game/FPS/Weapons/Sniper/SR_S96/Animations/SR_S96_Animations/AS_Weapon_SR_S96_Reload.AS_Weapon_SR_S96_Reload" false)
  (Rendering|SetVisibility (Variables|Default|GetAmmo_In_Magazine) false false)
  (Utilities|FlowControl|Delay 0.8)
  (Rendering|SetVisibility (Variables|Default|GetAmmo_In_Magazine) true false))

(event EventBeginPlay
  ;[1 1 1] Player Input
  (Input|EnableInput (Game|GetPlayerController 0)))

(event Input|KeyboardEvents|1
  (params (Key :type Key%20Structure :default "None"))
  (bind _sr_s96_skeletal (Variables|Default|GetSR_S96_Skeletal))
  (bind _returnvalue (Transformation|GetSocketRotation _sr_s96_skeletal "Shell_Socket"))
  (bind _returnvalue_2 (Math|Vector|GetRightVector _returnvalue))
  ;[1 1 1] Single Shoot
  (:Pressed
    (Components|Animation|PlayAnimation (Variables|Default|GetSR_S96_Skeletal) "/Game/FPS/Weapons/Sniper/SR_S96/Animations/SR_S96_Animations/AS_Weapon_SR_S96_Shoot.AS_Weapon_SR_S96_Shoot" false)
    ;[1 1 1] Bolt Chamber
    (Utilities|FlowControl|Delay 0.5)
    (Components|Animation|PlayAnimation (Variables|Default|GetSR_S96_Skeletal) "/Game/FPS/Weapons/Sniper/SR_S96/Animations/SR_S96_Animations/AS_Weapon_SR_S96_Bolt_Chamber.AS_Weapon_SR_S96_Bolt_Chamber" false)
    (Utilities|FlowControl|Delay 0.6)
    (bind _returnvalue_3 (Game|SpawnActorfromClass "/Game/FPS/Weapons/Sniper/SR_S96/Blueprints/BP_SR_S96_P_Shell.BP_SR_S96_P_Shell_C" (Math|Transform|MakeTransform (Transformation|GetSocketLocation _sr_s96_skeletal "Shell_Socket") _returnvalue "1.000000,1.000000,1.000000") "Undefined" 0 0))
    (Physics|AddImpulse (Variables|/Game/FPS/Weapons/Sniper/SR_S96/Blueprints/BP_SR_S96_P_Shell.BP_SR_S96_P_Shell_C|GetCase _returnvalue_3) (Math|Vector|MakeVector (.x _returnvalue_2) (+ (.y _returnvalue_2) 5e+01) (.z _returnvalue_2)) "Shell_Socket" false)
    (Transformation|AttachComponentToComponent _returnvalue_3 _sr_s96_skeletal "Shell_Socket" "SnapToTarget" "SnapToTarget" "SnapToTarget" true)
    (Components|Activation|Activate (Variables|Default|GetPS_SR_96_P_Extractor_Smoke) false)))

(event Input|KeyboardEvents|2
  (params (Key :type Key%20Structure :default "None"))
  ;[1 1 1] Reload
  (:Pressed
    (Components|Animation|PlayAnimation (Variables|Default|GetSR_S96_Skeletal) "/Game/FPS/Weapons/Sniper/SR_S96/Animations/SR_S96_Animations/AS_Weapon_SR_S96_Reload.AS_Weapon_SR_S96_Reload" false)
    (Rendering|SetVisibility (Variables|Default|GetAmmo_In_Magazine) false false)
    (Utilities|FlowControl|Delay 0.8)
    (Rendering|SetVisibility (Variables|Default|GetAmmo_In_Magazine) true false)))

(fn ConstructionScript)