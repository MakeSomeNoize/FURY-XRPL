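; Base Blueprint for spawnable submachine gun objects that drop to the floor as physics props.
; On begin play, the mesh starts simulating physics if the actor's owner class matches the weapon class.
; Hits play a drop sound and start a looping timer, unless one is running or the actor is frozen.
; The timer disables physics and freezes the actor once motion stops or about two seconds elapse.
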(event OnComponentHit(Mesh)
  (params (HitComponent :type Primitive%20Component%20Object%20Reference) (OtherActor :type Actor%20Object%20Reference) (OtherComp :type Primitive%20Component%20Object%20Reference) (NormalImpulse :type Vector :default "0, 0, 0") (Hit :type Hit%20Result%20Structure%20%28by%20ref%29))
  ;[1 1 1] On floor hit
  (if (and (not (Utilities|Time|IsTimerActivebyHandle (Variables|Default|GetIsBouncingCheckTimer))) (not (Variables|Default|GetIsFreezed?)))
    (Audio|PlaySoundatLocation (Variables|Default|GetDropSound) (.ImpactPoint (Collision|BreakHitResult Hit)) "0, 0, 0" 1.0 1.0 0.0 0 0 0 0)
    (bind _returnvalue (Utilities|Time|SetTimerbyEvent (delegate Custom|CheckIsBouncing) 0.1 true))
    (Variables|Default|SetIsBouncingCheckTimer _returnvalue)))

(event Custom|CheckIsBouncing
  ;[1 1 1] Check is bouncing after floor hit
  (if (or (and (== (Math|Vector|VectorLength (Physics|GetPhysicsAngularVelocityinDegrees (Variables|Default|GetMesh) "None")) 0.0) (== (Math|Vector|VectorLength (Transformation|GetVelocity)) 0.0)) (>= (Variables|Default|GetBouncingCheckTimerElapsed) 2.0))
    (Physics|SetSimulatePhysics (Variables|Default|GetMesh) false)
    (Utilities|Time|ClearandInvalidateTimerbyHandle (Variables|Default|GetIsBouncingCheckTimer))
    (Variables|Default|SetIsFreezed? true)
    (else
      (Variables|Default|SetBouncingCheckTimerElapsed (+ (Variables|Default|GetBouncingCheckTimerElapsed) 0.1)))))

(event EventBeginPlay
  ;[0.9698 1 0] Begin play
  (if (.IsInsideWeapon? (CallFunction|CheckifBelongstoWeapon))
    (Physics|SetSimulatePhysics (Variables|Default|GetMesh) true)))

(fn ConstructionScript
  (|CallParentFunction))

(fn CheckifBelongstoWeapon
  (bind _returnvalue (Components|GetOwner))
  (Utilities|IsValid _returnvalue
    (:Is%20Valid
      (LocalVariables|SetlIsInsideWeapon (== (Utilities|GetClass _returnvalue) (Variables|Default|GetWeaponClass))))
    (:Is%20Not%20Valid
      (LocalVariables|SetlIsInsideWeapon false)))
  (return (LocalVariables|GetlIsInsideWeapon) _returnvalue))