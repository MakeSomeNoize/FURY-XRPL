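; Base submachine gun weapon Blueprint that manages the visual skin of its registered mesh components: color theme and scratch intensity.
; The construction script and color theme setter call UpdateAppearance, which applies both settings.
; Preset themes swap materials by slot name from per-theme maps.
; Custom and Custom Camo reuse the Black and Desert materials, then override color vector parameters, while scratches use a scalar parameter.
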(event Custom|SetupMesh
  (params (MeshComponent :type Mesh%20Component%20Object%20Reference))
  ;[1 1 1] Setup appearance
  (Variables|Components|SetMeshComponents (Utilities|Array|MakeArray MeshComponent)))

(event Custom|UpdateAppearance
  ;[1 1 1] Update appearance
  (CallFunction|ChangeColorTheme (Variables|Appearance|GetColorTheme) (Variables|Appearance|GetCustomColor_01) (Variables|Appearance|GetCustomColor_02) (Variables|Appearance|GetCustomCamoColor_01) (Variables|Appearance|GetCustomCamoColor_02) (Variables|Appearance|GetCustomCamoColor_03) (Variables|Appearance|GetCustomCamoColor_04) (Variables|Appearance|GetCustomCamoColor_05) (Variables|Appearance|GetCustomCamoColor_06))
  (CallFunction|ChangeScratchIntensity (Variables|Appearance|GetScratchIntensity)))

(event Custom|SetupMeshes
  (params (MeshComponents :type Array%20of%20Mesh%20Component%20Object%20References))
  ;[1 1 1] Setup appearance
  (Variables|Components|SetMeshComponents MeshComponents))

(event EventSetColorTheme
  (params (ColorTheme :type E_DSMG_WeaponColorTheme%20Enum :default "NewEnumerator0") (OverwriteColors :type Boolean) (CustomColor_01 :type Linear%20Color%20Structure) (CustomColor_02 :type Linear%20Color%20Structure) (CustomCamoColor_01 :type Linear%20Color%20Structure) (CustomCamoColor_02 :type Linear%20Color%20Structure) (CustomCamoColor_03 :type Linear%20Color%20Structure) (CustomCamoColor_04 :type Linear%20Color%20Structure) (CustomCamoColor_05 :type Linear%20Color%20Structure) (CustomCamoColor_06 :type Linear%20Color%20Structure))
  ;[1 1 1] Set color theme
  (Variables|Appearance|SetColorTheme ColorTheme)
  (if OverwriteColors
    (Utilities|FlowControl|Sequence
      (:then_0
        (Variables|Appearance|SetCustomColor_01 CustomColor_01))
      (:then_1
        (Variables|Appearance|SetCustomColor_02 CustomColor_02))
      (:then_2
        (Variables|Appearance|SetCustomCamoColor_01 CustomCamoColor_01))
      (:then_3
        (Variables|Appearance|SetCustomCamoColor_02 CustomCamoColor_02))
      (:then_4
        (Variables|Appearance|SetCustomCamoColor_03 CustomCamoColor_03))
      (:then_5
        (Variables|Appearance|SetCustomCamoColor_04 CustomCamoColor_04))
      (:then_6
        (Variables|Appearance|SetCustomCamoColor_05 CustomCamoColor_05))
      (:then_7
        (Variables|Appearance|SetCustomCamoColor_06 CustomCamoColor_06))
      (:then_8
        (CallFunction|UpdateAppearance :!label _label)))
    (else
      (goto _label))))

(event EventSetScratchIntensity
  (params (ScratchIntensity :type Float%20%28double-precision%29))
  ;[1 1 1] Set scratch intensity
  (bind _output_get (Variables|Appearance|SetScratchIntensity ScratchIntensity))
  (CallFunction|ChangeScratchIntensity _output_get))

(fn ConstructionScript
  (CallFunction|UpdateAppearance))

(fn ChangeColorTheme
  (params (ColorTheme :type E_DSMG_WeaponColorTheme%20Enum :default "NewEnumerator0") (CustomColor_01 :type Linear%20Color%20Structure) (CustomColor_02 :type Linear%20Color%20Structure) (CustomCamoColor_01 :type Linear%20Color%20Structure) (CustomCamoColor_02 :type Linear%20Color%20Structure) (CustomCamoColor_03 :type Linear%20Color%20Structure) (CustomCamoColor_04 :type Linear%20Color%20Structure) (CustomCamoColor_05 :type Linear%20Color%20Structure) (CustomCamoColor_06 :type Linear%20Color%20Structure))
  (bind _materials (Variables|Appearance|GetMaterials))
  (bind _materials_2 (Variables|Appearance|GetMaterials))
  (bind (_black _desert) (Utilities|Struct|BreakST_DSMG_WeaponMaterials _materials_2))
  (if (> (Utilities|Array|Length (Variables|Components|GetMeshComponents)) 0)
    (switch Utilities|FlowControl|Switch|SwitchonE_DSMG_WeaponColorTheme ColorTheme
      (:NewEnumerator0
        ;[1 1 1] Set predefined color themes
        (Utilities|SetMaterialsbyMap (.black _materials)))
      (:NewEnumerator1
        (Utilities|SetMaterialsbyMap (.desert _materials)))
      (:NewEnumerator2
        (Utilities|SetMaterialsbyMap (.modern _materials)))
      (:NewEnumerator3
        (Utilities|SetMaterialsbyMap (.sienna _materials)))
      (:NewEnumerator4
        (Utilities|SetMaterialsbyMap (.winter _materials)))
      (:NewEnumerator5
        (Utilities|SetMaterialsbyMap (.wood _materials)))
      (:NewEnumerator6
        ;[1 1 1] Set monochrome custom colors
        (Utilities|SetMaterialsbyMap _black)
        (Utilities|SetCustomColorsbyMap (Utilities|Map|MakeMap "Color_01" CustomColor_01 "Color_02" CustomColor_02)))
      (:NewEnumerator7
        ;[1 1 1] Set camo custom colors
        (Utilities|SetMaterialsbyMap _desert)
        (Utilities|SetCustomColorsbyMap (Utilities|Map|MakeMap "CamoColor_01" CustomCamoColor_01 "CamoColor_02" CustomCamoColor_02 "CamoColor_03" CustomCamoColor_03 "CamoColor_04" CustomCamoColor_04 "CamoColor_05" CustomCamoColor_05 "CamoColor_06" CustomCamoColor_06))))))

(fn ChangeScratchIntensity
  (params (ScratchIntensity :type Float%20%28double-precision%29))
  (for _array_element (Variables|Components|GetMeshComponents)
    (Utilities|IsValid _array_element
      (:Is%20Valid
        (Rendering|Material|SetScalarParameterValueonMaterials _array_element "ScratchIntensity" ScratchIntensity)))))

(fn GetColorTheme
  (return (Variables|Appearance|GetColorTheme) (Variables|Appearance|GetCustomColor_01) (Variables|Appearance|GetCustomColor_02) (Variables|Appearance|GetCustomCamoColor_01) (Variables|Appearance|GetCustomCamoColor_02) (Variables|Appearance|GetCustomCamoColor_03) (Variables|Appearance|GetCustomCamoColor_04) (Variables|Appearance|GetCustomCamoColor_05) (Variables|Appearance|GetCustomCamoColor_06)))

(fn GetScratchIntensity
  (return (Variables|Appearance|GetScratchIntensity)))