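; Magazine actor Blueprint for the DSMG submachine gun, swapping between full and empty static meshes.
; Construction applies the ammo-state mesh and runs mesh setup.
; On BeginPlay, if it belongs to a weapon, it switches to the empty mesh and copies the owning weapon's color theme and scratch intensity.
; It also re-aligns rotation and mesh offset so the WeaponSocket acts as its pivot.
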(event Custom|SetAmmoState
  (params (IsEmpty? :type Boolean))
  (bind _mesh (Variables|Character|GetMesh))
  ;[1 1 1] Ammo variants
  (if IsEmpty?
    (Components|StaticMesh|SetStaticMesh _mesh (Variables|Default|GetStaticMeshEmpty))
    (else
      (Components|StaticMesh|SetStaticMesh _mesh (Variables|Default|GetStaticMeshFull)))))

(event EventBeginPlay
  (bind (_isinsideweapon_ _owner) (CallFunction|CheckifBelongstoWeapon))
  ;[0.9698 1 0] Begin play
  (|CallParentFunction)
  (if _isinsideweapon_
    (CallFunction|MatchPivottoSocket "WeaponSocket")
    (CallFunction|SetAmmoState true)
    (bind _asbp_dsmg_base_weapon (Utilities|Casting|CastToBP_DSMG_BaseWeapon _owner))
    (bind (_colortheme _customcolor_01 _customcolor_02 _customcamocolor_01 _customcamocolor_02 _customcamocolor_03 _customcamocolor_04 _customcamocolor_05 _customcamocolor_06) (Default|GetColorTheme _asbp_dsmg_base_weapon))
    (CallFunction|SetColorTheme _colortheme true _customcolor_01 _customcolor_02 _customcamocolor_01 _customcamocolor_02 _customcamocolor_03 _customcamocolor_04 _customcamocolor_05 _customcamocolor_06)
    (bind _scratchintensity (Default|GetScratchIntensity _asbp_dsmg_base_weapon))
    (CallFunction|SetScratchIntensity _scratchintensity)))

(fn ConstructionScript
  (CallFunction|SetAmmoState (Variables|Appearance|GetIsEmpty?))
  (CallFunction|SetupMesh (Variables|Character|GetMesh))
  (|CallParentFunction))

(fn MatchPivottoSocket
  (params (InSocketName :type Name))
  (bind _mesh (Variables|Character|GetMesh))
  (Transformation|SetActorRotation (Math|Rotator|Delta(Rotator) (Class|KismetMathLibrary|NegateRotator (.rotation (Transformation|GetSocketTransform _mesh InSocketName "RTS_Component"))) (Transformation|GetActorRotation)))
  (Transformation|AddWorldOffset (Variables|Character|GetMesh) (- (Transformation|GetWorldLocation _mesh) (Transformation|GetSocketLocation _mesh InSocketName)) false false))