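; Submachine gun weapon actor that binds to its parent character's fire and action events to manage ammo, montages and sound.
; Firing cycles chamber and magazine counts and rotates shot audio components, whose playback position offsets the tail sound on release; projectile spawning is disconnected.
; Color theme and scratch changes propagate to attachments.
; Audio booleans are set by rewriting default parameters, a temporary UE5 bug workaround.
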(event OnAudioPlaybackPercent(Shot_01)
  (params (PlayingSoundWave :type Sound%20Wave%20Object%20Reference) (PlaybackPercent :type Float%20%28single-precision%29))
  ;[1 1 1] Play sounds
  (Audio|SaveShotPlaybackTime 0 PlayingSoundWave PlaybackPercent))

(event OnAudioPlaybackPercent(Shot_04)
  (params (PlayingSoundWave :type Sound%20Wave%20Object%20Reference) (PlaybackPercent :type Float%20%28single-precision%29))
  ;[1 1 1] Play sounds
  (Audio|SaveShotPlaybackTime 3 PlayingSoundWave PlaybackPercent))

(event OnAudioPlaybackPercent(Shot_02)
  (params (PlayingSoundWave :type Sound%20Wave%20Object%20Reference) (PlaybackPercent :type Float%20%28single-precision%29))
  ;[1 1 1] Play sounds
  (Audio|SaveShotPlaybackTime 1 PlayingSoundWave PlaybackPercent))

(event OnAudioPlaybackPercent(Shot_03)
  (params (PlayingSoundWave :type Sound%20Wave%20Object%20Reference) (PlaybackPercent :type Float%20%28single-precision%29))
  ;[1 1 1] Play sounds
  (Audio|SaveShotPlaybackTime 2 PlayingSoundWave PlaybackPercent))

(event Custom|LoadCaliber
  ;[1 1 1] Load / unload caliber
  (if (and (not (CallFunction|CheckIsLoaded)) (not (CallFunction|CheckIsMagazineEmpty)))
    (bind _result (Math|Integer|DecrementInt (CallFunction|GetMagazineAmmo))
      (:%20%20
        (CallFunction|SetAmmo 1 _result true)))))

(event Custom|RefillAmmo
  ;[1 1 1] Refill ammo
  (CallFunction|SetAmmo (Math|Conversions|ToInteger(Boolean) (CallFunction|CheckIsLoaded)) (Variables|Default|GetCapacity) false))

(event Custom|HandleActionChanged
  (params (Action :type E_DSMG_CharacterAction%20Enum :default "NewEnumerator9") (AnimIndex :type Integer) (BlendInTime :type Float%20%28double-precision%29) (BlendOutTime :type Float%20%28double-precision%29))
  ;[1 1 1] Action changed
  (Animations|PlayActionMontage Action AnimIndex BlendInTime BlendOutTime))

(event Custom|SpawnBulletShell
  ;[1 1 1] Spawn parts
  (Game|SpawnActorfromClass (Variables|Default|GetBulletShellClass) (Math|Transform|MakeTransform (+ (* (Transformation|GetActorRightVector) (Math|Float|MakeLiteralFloat 1.5e+02)) (Transformation|GetActorLocation)) (.rotation (Transformation|GetSocketTransform (Variables|Default|GetRifle) "bullet_shell" "RTS_Actor"))) "AlwaysSpawn" self 0))

(event Custom|Reload
  (Animations|PlayActionMontage "NewEnumerator0" 0 0.2 0.4))

(event Custom|PlayMoveBoltSound
  (params (IsPulled? :type Boolean) (IsShortMotion? :type Boolean))
  ;[1 1 1] Play sounds
  (Utilities|SetBooleanParameterFix (Variables|Default|GetBoltAction) "IsPulled?" IsPulled?)
  (Utilities|SetBooleanParameterFix (Variables|Default|GetBoltAction) "IsShortMotion?" IsShortMotion?)
  (Audio|Components|Audio|Play (Variables|Default|GetBoltAction) 0.0))

(event Custom|HandleFireStarted
  ;[1 1 1] Fire
  (if (> (CallFunction|GetAmmo) 0)
    (CallFunction|PlayShotSound)
    (if (CallFunction|CheckIsLastCaliber)
      (CallFunction|PlayShotTailSound 0.03))
    (if (CallFunction|CheckIsLoaded)
      (CallFunction|UnloadCaliber)
      (CallFunction|LoadCaliber)
      (else
        (CallFunction|SetAmmo (Math|Conversions|ToInteger(Boolean) (CallFunction|CheckIsLoaded)) (CallFunction|GetMagazineAmmo) false)))))

(event Custom|PlayShotSound
  ;[1 1 1] Play sounds
  (bind _shotcomponent (Audio|GetShotComponentbyIndex (Variables|Audio|GetNextShotIndex)))
  (Utilities|SetBooleanParameterFix _shotcomponent "IsSilenced?" (Variables|Default|GetIsSilenced?))
  (Audio|Components|Audio|Play _shotcomponent 0.0)
  (Variables|Audio|SetCurrentShotIndex (Variables|Audio|GetNextShotIndex))
  (if (Audio|CheckIsLastShotComponentbyIndex (Variables|Audio|GetNextShotIndex))
    (Variables|Audio|SetNextShotIndex 0)
    (else
      (Math|Integer|IncrementInt (Variables|Audio|GetNextShotIndex)))))

(event Custom|PlayShotTailSound
  (params (StartTime :type Float%20%28double-precision%29))
  ;[1 1 1] Play sounds
  (Utilities|SetBooleanParameterFix (Variables|Default|GetShotTail) "IsSilenced?" (Variables|Default|GetIsSilenced?))
  (Audio|Components|Audio|Play (Variables|Default|GetShotTail) StartTime))

(event Custom|HandleActionInterrupted
  (params (InBlendOutTime :type Float%20%28double-precision%29))
  (bind _rifle (Variables|Default|GetRifle))
  (bind _returnvalue (Components|SkeletalMesh|GetAnimInstance _rifle))
  ;[1 1 1] Action interrupted
  (Utilities|IsValid _returnvalue
    (:Is%20Valid
      (if (Animation|Montage|MontageIsPlaying _returnvalue (Variables|Animations|GetCurrentActionMontage))
        (Animation|Montage|MontageStop _returnvalue InBlendOutTime (Variables|Animations|GetCurrentActionMontage))))))

(event Custom|ToggleSilencer
  ;[1 1 1] Toggle silencer sounds
  (Variables|Default|SetIsSilenced? (not (Variables|Default|GetIsSilenced?))))

(event Custom|EmitBoltPowderGas
  ;[1 1 1] Emit particle effects
)

(event Custom|EmitMuzzleFlash
  ;[1 1 1] Emit particle effects
  (Effects|SpawnEmitterAttached "/Game/FPS/Weapons/SubmachineGun/Particles/PS_MuzzleFlash.PS_MuzzleFlash" (Variables|Default|GetRifle) (Utilities|Name|MakeLiteralName "MuzzleFlashSocket") "0, 0, 0" "0, 0, 0" "1.000000,1.000000,1.000000" "SnapToTarget"))

(event Custom|HandleFireReleased
  (params (IsByPlayer? :type Boolean))
  ;[1 1 1] Fire
  (if (and IsByPlayer? (> (CallFunction|GetAmmo) 0))
    (CallFunction|PlayShotTailSound (Variables|Audio|GetShotPlaybackTime))))

(event Custom|ChangeGrip
  (params (Grip :type E_DSMG_WeaponGrip%20Enum :default "NewEnumerator0"))
  ;[1 1 1] Change grip
  (bind _output_get (Variables|Appearance|SetGrip Grip))
  (Default|CallOnGripChanged _output_get))

(event Custom|SpawnMagazine
  (bind _rifle (Variables|Default|GetRifle))
  (bind _returnvalue (Transformation|GetSocketTransform _rifle "magazine" "RTS_World"))
  ;[1 1 1] Spawn parts
  (bind _returnvalue_2 (Game|SpawnActorfromClass (Variables|Default|GetMagazineClass) (Math|Transform|MakeTransform (.location _returnvalue) (.rotation _returnvalue)) "AlwaysSpawn" self 0))
  (Utilities|FlowControl|Delay 2e+01)
  (Actor|DestroyActor _returnvalue_2))

(event Custom|UnloadCaliber
  ;[1 1 1] Load / unload caliber
  (CallFunction|SetAmmo 0 (CallFunction|GetMagazineAmmo) (Variables|Default|GetIsCocked?)))

(event EventDestroyed
  ;[0 0 0] Destroyed
  (bind _asbp_dsmg_character (Utilities|CasttoCharacter))
  (EventDispatchers|UnbindEventfromOnFireStarted _asbp_dsmg_character (delegate Custom|HandleFireStarted))
  (EventDispatchers|UnbindEventfromOnFireReleased _asbp_dsmg_character (delegate Custom|HandleFireReleased))
  (EventDispatchers|UnbindEventfromOnActionChanged _asbp_dsmg_character (delegate Custom|HandleActionChanged))
  (EventDispatchers|UnbindEventfromOnActionInterrupted _asbp_dsmg_character (delegate Custom|HandleActionInterrupted)))

(event EventChangeColorTheme
  (params (ColorTheme :type E_DSMG_WeaponColorTheme%20Enum :default "NewEnumerator0") (CustomColor_01 :type Linear%20Color%20Structure) (CustomColor_02 :type Linear%20Color%20Structure) (CustomCamoColor_01 :type Linear%20Color%20Structure) (CustomCamoColor_02 :type Linear%20Color%20Structure) (CustomCamoColor_03 :type Linear%20Color%20Structure) (CustomCamoColor_04 :type Linear%20Color%20Structure) (CustomCamoColor_05 :type Linear%20Color%20Structure) (CustomCamoColor_06 :type Linear%20Color%20Structure))
  ;[1 1 1] Override ChangeColorTheme to drive color theme for attachments
  (|CallParentFunction ColorTheme CustomColor_01 CustomColor_02 CustomCamoColor_01 CustomCamoColor_02 CustomCamoColor_03 CustomCamoColor_04 CustomCamoColor_05 CustomCamoColor_06)
  (for _array_element (CallFunction|GetAttachments)
    (Utilities|IsValid (Variables|/Script/Engine.ChildActorComponent|GetChildActor _array_element)
      (:Is%20Valid
        (if (Utilities|Enum|Equal(Enum) (Utilities|GetObjectName _array_element) "IronSights")
          (if (Utilities|Enum|Equal(Enum) ColorTheme "NewEnumerator7")
            (Class|BPIDSMGWeapon|SetColorTheme(Message) (Variables|/Script/Engine.ChildActorComponent|GetChildActor _array_element) "NewEnumerator6" true CustomCamoColor_01)
            (else
              (Class|BPIDSMGWeapon|SetColorTheme(Message) (Variables|/Script/Engine.ChildActorComponent|GetChildActor _array_element) ColorTheme true CustomColor_01 CustomColor_02 CustomCamoColor_01 CustomCamoColor_02 CustomCamoColor_03 CustomCamoColor_04 CustomCamoColor_05 CustomCamoColor_06 :!label _label)))
          (else
            (goto _label)))))))

(event EventChangeScratchIntensity
  (params (ScratchIntensity :type Float%20%28double-precision%29))
  ;[1 1 1] Override ChangeScratchIntensity to drive scratch intensity for attachments
  (|CallParentFunction ScratchIntensity)
  (for _array_element (CallFunction|GetAttachments)
    (Utilities|IsValid (Variables|/Script/Engine.ChildActorComponent|GetChildActor _array_element)
      (:Is%20Valid
        (Class|BPIDSMGWeapon|SetScratchIntensity(Message) (Variables|/Script/Engine.ChildActorComponent|GetChildActor _array_element) ScratchIntensity)))))

(event EventBeginPlay
  ;[0.9698 1 0] Begin play
  (CallFunction|SetAmmo 0 (Variables|Default|GetCapacity) false)
  (bind _asbp_dsmg_character (Utilities|CasttoCharacter))
  (EventDispatchers|BindEventtoOnFireStarted _asbp_dsmg_character (delegate Custom|HandleFireStarted))
  (EventDispatchers|AssignOnFireReleased _asbp_dsmg_character (delegate Custom|HandleFireReleased))
  (EventDispatchers|BindEventtoOnActionChanged _asbp_dsmg_character (delegate Custom|HandleActionChanged))
  (EventDispatchers|BindEventtoOnActionInterrupted _asbp_dsmg_character (delegate Custom|HandleActionInterrupted)))

(fn ConstructionScript
  (CallFunction|SetupMesh (Variables|Default|GetRifle))
  (|CallParentFunction))

(fn GetStats
  (return (Utilities|String|EnumtoString (Variables|Default|GetColorTheme)) (Utilities|String|ToString(Float) (Variables|Default|GetScratchIntensity)) (Utilities|String|EnumtoString (Variables|Appearance|GetGrip)) (Utilities|String|SelectString "Silenced" "Loud" (Variables|Default|GetIsSilenced?)) (Utilities|String|Append (Utilities|String|ToString(Integer) (CallFunction|GetMagazineAmmo)) "/" (Utilities|String|ToString(Integer) (Variables|Default|GetCapacity)) (Utilities|String|SelectString " +1" "" (CallFunction|CheckIsLoaded)))))

(fn ChangeSteppedScratchIntensity
  (params (Increment? :type Boolean) (Step :type Float%20%28double-precision%29))
  (bind _scratchintensity (Variables|Default|GetScratchIntensity))
  (bind _scratchintensity_2 (Variables|Default|GetScratchIntensity))
  (bind _returnvalue (- _scratchintensity Step))
  (bind _returnvalue_2 (+ _scratchintensity_2 Step))
  (if Increment?
    (Math|Float|CompareFloat _returnvalue_2 1.0
      (:>
        (LocalVariables|SetlScratchIntensity 1.0))
      (:==
        (LocalVariables|SetlScratchIntensity _returnvalue_2 :!label _label))
      (:<
        (goto _label)))
    (else
      (Math|Float|CompareFloat _returnvalue 0.0
        (:>
          (LocalVariables|SetlScratchIntensity _returnvalue :!label _label_2))
        (:==
          (goto _label_2))
        (:<
          (LocalVariables|SetlScratchIntensity 0.0)))))
  (CallFunction|SetScratchIntensity (LocalVariables|GetlScratchIntensity)))

(fn GetAimVerticalOffset
  (bind _ironsights (Variables|Default|GetIronSights))
  (bind _childactor (Variables|/Script/Engine.ChildActorComponent|GetChildActor _ironsights))
  (Utilities|IsValid _childactor
    (:Is%20Valid
      (bind _asbp_dsmg_iron_sights (Utilities|Casting|CastToBP_DSMG_IronSights _childactor))
      (bind _verticaloffset (Default|GetAimVerticalOffset _asbp_dsmg_iron_sights))
      (return _verticaloffset))))

(fn GetAttachments
  (return (Utilities|Array|MakeArray (Variables|Default|GetHandStop) (Variables|Default|GetStock) (Variables|Default|GetIronSights) (Variables|Default|GetPicatinny))))

(fn PlayActionMontage
  (params (Action :type E_DSMG_CharacterAction%20Enum :default "NewEnumerator9") (AnimIndex :type Integer) (BlendInTime :type Float%20%28double-precision%29) (BlendOutTime :type Float%20%28double-precision%29))
  (bind _reloademptyanimations (Variables|Animations|GetReloadEmptyAnimations))
  (switch Utilities|FlowControl|Switch|SwitchonE_DSMG_CharacterAction Action
    (:NewEnumerator0
      (if (CallFunction|CheckIsLoaded)
        (LocalVariables|SetlAnimSequence (Utilities|Array|Get(acopy) _reloademptyanimations))
        (else
          (LocalVariables|SetlAnimSequence (Utilities|Array|Get(acopy) _reloademptyanimations AnimIndex))))
      (bind _returnvalue (Class|AnimInstance|PlaySlotAnimationasDynamicMontage (Components|SkeletalMesh|GetAnimInstance (Variables|Default|GetRifle)) (LocalVariables|GetlAnimSequence) "DefaultSlot" BlendInTime BlendOutTime 1.0 1 -1.0 0.0 :!label _label))
      (Variables|Animations|SetCurrentActionMontage _returnvalue))
    (:NewEnumerator3
      (LocalVariables|SetlAnimSequence (Utilities|Array|Get(acopy) (Variables|Animations|GetBoltActionAnimations) AnimIndex))
      (goto _label))
    (:NewEnumerator10
      (LocalVariables|SetlAnimSequence (Utilities|Array|Get(acopy) (Variables|Animations|GetCheckAmmoAnimations) AnimIndex))
      (goto _label))
    (:NewEnumerator12
      (LocalVariables|SetlAnimSequence (Utilities|Array|Get(acopy) (Variables|Animations|GetCheckMagazineAnimations) AnimIndex))
      (goto _label))
    (:NewEnumerator13
      (if (== AnimIndex 0)
        (LocalVariables|SetlAnimSequence (Utilities|Array|Get(acopy) (Variables|Animations|GetCheckChamberAnimations) AnimIndex))
        (goto _label)))))

(fn GetFireRate
  (return (Variables|Default|GetFireRate)))

(fn SaveShotPlaybackTime
  (params (ShotIndex :type Integer) (PlayingSoundWave :type Sound%20Base%20Object%20Reference) (PlaybackPercent :type Float%20%28double-precision%29))
  (if (== ShotIndex (Variables|Audio|GetCurrentShotIndex))
    (Variables|Audio|SetShotPlaybackTime (* (Variables|/Script/Engine.SoundBase|GetDuration PlayingSoundWave) PlaybackPercent))))

(fn GetShotComponentbyIndex
  (params (ShotIndex :type Integer))
  (bind _shots (Variables|Default|GetShots))
  (bind _children (Components|GetChildrenComponents _shots false))
  (bind _output (Utilities|Array|Get(acopy) _children ShotIndex))
  (Utilities|IsValid _output
    (:Is%20Valid
      (bind _asaudio_component (Utilities|Casting|CastToAudioComponent _output))
      (return _asaudio_component))))

(fn CheckIsLastShotComponentbyIndex
  (params (ShotIndex :type Integer))
  (return (== ShotIndex (Utilities|Array|LastIndex (Components|GetChildrenComponents (Variables|Default|GetShots) false)))))

(fn SetAmmo
  (params (Chamber :type Integer) (Magazine :type Integer) (IsCocked? :type Boolean))
  (Variables|Default|SetAmmo (Utilities|Array|MakeArray Chamber Magazine))
  (bind _output_get (Variables|Default|SetIsCocked? IsCocked?))
  (Default|CallOnAmmoChanged (CallFunction|GetMagazineAmmo) (Variables|Default|GetCapacity) (CallFunction|CheckIsLoaded) _output_get))

(fn GetAmmo
  (bind _ammo (Variables|Default|GetAmmo))
  (return (+ (Utilities|Array|Get(acopy) _ammo) (Utilities|Array|Get(acopy) _ammo 1))))

(fn GetMagazineAmmo
  (return (Utilities|Array|Get(acopy) (Variables|Default|GetAmmo) 1)))

(fn CheckIsLoaded
  (return (== (Utilities|Array|Get(acopy) (Variables|Default|GetAmmo)) 1)))

(fn CheckIsMagazineEmpty
  (return (== (Utilities|Array|Get(acopy) (Variables|Default|GetAmmo) 1) 0)))

(fn CheckIsLastCaliber
  (return (== (CallFunction|GetAmmo) 1)))

(fn GetReloadEmptyAnimationsLastIndex
  (return (Utilities|Array|LastIndex (Variables|Animations|GetReloadEmptyAnimations))))

(fn SetBoltCatchedState
  (params (IsBoltCatched? :type Boolean))
  (bind _output_get (Variables|Default|SetIsBoltCatched? IsBoltCatched?))
  (Default|CallOnBoltCatchedChanged _output_get))