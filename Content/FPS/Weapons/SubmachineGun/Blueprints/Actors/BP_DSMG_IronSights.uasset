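; BP_DSMG_IronSights is an iron sights actor for the submachine gun, built from Rear and Front sight components.
; Its construction script passes both components to SetupMeshes, applies the stored front sight offset, then runs the parent construction script.
; The ChangeFrontOffset event stores a new offset and moves the front sight along its relative X axis, so the spacing between sights is adjustable.
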(event Custom|ChangeFrontOffset
  (params (Offset :type Float%20%28double-precision%29))
  ;[1 1 1] Change front sight offset
  (bind _output_get (Variables|Default|SetFrontSightOffset Offset))
  (Transformation|SetRelativeLocation (Variables|Default|GetFront) (Math|Vector|MakeVector _output_get 0.0 0.0) false false))

(fn ConstructionScript
  (CallFunction|SetupMeshes (Utilities|Array|MakeArray (Variables|Default|GetRear) (Variables|Default|GetFront)))
  (CallFunction|ChangeFrontOffset (Variables|Default|GetFrontSightOffset))
  (|CallParentFunction))