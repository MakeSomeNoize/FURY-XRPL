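; First-person hands actor that demos the CS-34 SMG animation set through hard-coded keyboard keys.
; The equip key spawns BP_CS_34_SMG once, attaches it to the hand socket and disables its input.
; Keys play hand animations directly, using delays to return most to idle and to loop full-auto fire.
; Several also call matching Hands events on the weapon, found through GetAllActorsOfClass.
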(event EventBeginPlay
  ;[1 1 1] Player Input
  (Input|EnableInput (Game|GetPlayerController 0)))

(event Input|KeyboardEvents|4
  (params (Key :type Key%20Structure))
  ;[1 1 1] Shooting
  (:Pressed
    (if (Variables|Default|GetWeapon%20is%20Spawned)
      (bind _outactors (Actor|GetAllActorsOfClass "/Game/FPS/Weapons/SubmachineGun/CS_34_Smg/Blueprints/BP_CS_34_SMG.BP_CS_34_SMG_C"))
      (Default|HandsSooting (Utilities|Array|Get(acopy) _outactors)))
    (Components|Animation|PlayAnimation (Variables|Default|GetHands) "/Game/FPS/Weapons/SubmachineGun/CS_34_Smg/Animations/Hand_Animations/AS_Hands_CS_34_Shooting.AS_Hands_CS_34_Shooting" false)
    (Utilities|FlowControl|Delay 0.5)
    (Components|Animation|PlayAnimation (Variables|Default|GetHands) "/Game/FPS/Weapons/SubmachineGun/CS_34_Smg/Animations/Hand_Animations/AS_Hands_CS_34_Idle.AS_Hands_CS_34_Idle" false)))

(event Input|KeyboardEvents|5
  (params (Key :type Key%20Structure))
  ;[1 1 1] Reload
  (:Pressed
    (if (Variables|Default|GetWeapon%20is%20Spawned)
      (bind _outactors (Actor|GetAllActorsOfClass "/Game/FPS/Weapons/SubmachineGun/CS_34_Smg/Blueprints/BP_CS_34_SMG.BP_CS_34_SMG_C"))
      (Default|HandsReloading (Utilities|Array|Get(acopy) _outactors)))
    (Components|Animation|PlayAnimation (Variables|Default|GetHands) "/Game/FPS/Weapons/SubmachineGun/CS_34_Smg/Animations/Hand_Animations/AS_Hands_CS_34_Reload.AS_Hands_CS_34_Reload" false)
    (Utilities|FlowControl|Delay 2.133)
    (Components|Animation|PlayAnimation (Variables|Default|GetHands) "/Game/FPS/Weapons/SubmachineGun/CS_34_Smg/Animations/Hand_Animations/AS_Hands_CS_34_Idle.AS_Hands_CS_34_Idle" true)))

(event Input|KeyboardEvents|9
  (params (Key :type Key%20Structure))
  ;[1 1 1] Scope Aim
  (:Pressed
    (Components|Animation|PlayAnimation (Variables|Default|GetHands) "/Game/FPS/Weapons/SubmachineGun/CS_34_Smg/Animations/Hand_Animations/AS_Hands_CS_34_Aim.AS_Hands_CS_34_Aim" false)))

(event Input|KeyboardEvents|0
  (params (Key :type Key%20Structure))
  ;[1 1 1] Aim Shoot
  (:Pressed
    (if (Variables|Default|GetWeapon%20is%20Spawned)
      (Variables|Default|SetFull%20Auto%20Shooting true)
      (bind _outactors (Actor|GetAllActorsOfClass "/Game/FPS/Weapons/SubmachineGun/CS_34_Smg/Blueprints/BP_CS_34_SMG.BP_CS_34_SMG_C"))
      (Default|HandsFullAutoShoot (Utilities|Array|Get(acopy) _outactors)))
    (Components|Animation|PlayAnimation (Variables|Default|GetHands) "/Game/FPS/Weapons/SubmachineGun/CS_34_Smg/Animations/Hand_Animations/AS_Hands_CS_34_AimShoot.AS_Hands_CS_34_AimShoot" false :!label _label)
    (Utilities|FlowControl|Delay 0.08)
    (if (Variables|Default|GetFull%20Auto%20Shooting)
      (goto _label)))
  (:Released
    (bind _outactors_2 (Actor|GetAllActorsOfClass "/Game/FPS/Weapons/SubmachineGun/CS_34_Smg/Blueprints/BP_CS_34_SMG.BP_CS_34_SMG_C"))
    (Default|HandsStopFullAutoShooting (Utilities|Array|Get(acopy) _outactors_2))
    (Utilities|FlowControl|Delay 0.1)
    (Variables|Default|SetFull%20Auto%20Shooting false)))

(event Input|KeyboardEvents|6
  (params (Key :type Key%20Structure))
  ;[1 1 1] Shooting Full Auto
  (:Pressed
    (if (Variables|Default|GetWeapon%20is%20Spawned)
      (Variables|Default|SetFull%20Auto%20Shooting true)
      (bind _outactors (Actor|GetAllActorsOfClass "/Game/FPS/Weapons/SubmachineGun/CS_34_Smg/Blueprints/BP_CS_34_SMG.BP_CS_34_SMG_C"))
      (Default|HandsFullAutoShoot (Utilities|Array|Get(acopy) _outactors)))
    (Components|Animation|PlayAnimation (Variables|Default|GetHands) "/Game/FPS/Weapons/SubmachineGun/CS_34_Smg/Animations/Hand_Animations/AS_Hands_CS_34_Shooting.AS_Hands_CS_34_Shooting" false :!label _label)
    (Utilities|FlowControl|Delay 0.08)
    (if (Variables|Default|GetFull%20Auto%20Shooting)
      (goto _label)))
  (:Released
    (bind _outactors_2 (Actor|GetAllActorsOfClass "/Game/FPS/Weapons/SubmachineGun/CS_34_Smg/Blueprints/BP_CS_34_SMG.BP_CS_34_SMG_C"))
    (Default|HandsStopFullAutoShooting (Utilities|Array|Get(acopy) _outactors_2))
    (Utilities|FlowControl|Delay 0.1)
    (Variables|Default|SetFull%20Auto%20Shooting false)
    (Utilities|FlowControl|Delay 0.2)
    (Components|Animation|PlayAnimation (Variables|Default|GetHands) "/Game/FPS/Weapons/SubmachineGun/CS_34_Smg/Animations/Hand_Animations/AS_Hands_CS_34_Idle.AS_Hands_CS_34_Idle" false)))

(event Input|KeyboardEvents|Hyphen
  (params (Key :type Key%20Structure))
  (bind _hands (Variables|Default|GetHands))
  ;[1 1 1] Scope UnAim
  (:Pressed
    (Components|Animation|PlayAnimation _hands "/Game/FPS/Weapons/SubmachineGun/CS_34_Smg/Animations/Hand_Animations/AS_Hands_CS_34_UnAim.AS_Hands_CS_34_UnAim" false)
    (Utilities|FlowControl|Delay 0.427)
    (Components|Animation|PlayAnimation _hands "/Game/FPS/Weapons/SubmachineGun/CS_34_Smg/Animations/Hand_Animations/AS_Hands_CS_34_Idle.AS_Hands_CS_34_Idle" true)))

(event Input|KeyboardEvents|Equals
  (params (Key :type Key%20Structure))
  ;[1 1 1] Weapon unequip
  (:Pressed
    (if (Variables|Default|GetWeapon%20is%20Spawned)
      (bind _outactors (Actor|GetAllActorsOfClass "/Game/FPS/Weapons/SubmachineGun/CS_34_Smg/Blueprints/BP_CS_34_SMG.BP_CS_34_SMG_C"))
      (Default|HandsUnequip (Utilities|Array|Get(acopy) _outactors))
      (Components|Animation|PlayAnimation (Variables|Default|GetHands) "/Game/FPS/Weapons/SubmachineGun/CS_34_Smg/Animations/Hand_Animations/AS_Hands_CS_34_UnEquip.AS_Hands_CS_34_UnEquip" false))))

(event Input|KeyboardEvents|7
  (params (Key :type Key%20Structure))
  ;[1 1 1] FullReload
  (:Pressed
    (if (Variables|Default|GetWeapon%20is%20Spawned)
      (bind _outactors (Actor|GetAllActorsOfClass "/Game/FPS/Weapons/SubmachineGun/CS_34_Smg/Blueprints/BP_CS_34_SMG.BP_CS_34_SMG_C"))
      (Default|HandsFullReload (Utilities|Array|Get(acopy) _outactors)))
    (Components|Animation|PlayAnimation (Variables|Default|GetHands) "/Game/FPS/Weapons/SubmachineGun/CS_34_Smg/Animations/Hand_Animations/AS_Hands_CS_34_FullReload.AS_Hands_CS_34_FullReload" false)
    (Utilities|FlowControl|Delay 2.133)
    (Components|Animation|PlayAnimation (Variables|Default|GetHands) "/Game/FPS/Weapons/SubmachineGun/CS_34_Smg/Animations/Hand_Animations/AS_Hands_CS_34_Idle.AS_Hands_CS_34_Idle" true)))

(event Input|KeyboardEvents|3
  (params (Key :type Key%20Structure))
  (bind _hands (Variables|Default|GetHands))
  ;[1 1 1] Running
  (:Pressed
    (Components|Animation|PlayAnimation _hands "/Game/FPS/Weapons/SubmachineGun/CS_34_Smg/Animations/Hand_Animations/AS_Hands_CS_34_Running.AS_Hands_CS_34_Running" true))
  (:Released
    (Components|Animation|PlayAnimation _hands "/Game/FPS/Weapons/SubmachineGun/CS_34_Smg/Animations/Hand_Animations/AS_Hands_CS_34_Idle.AS_Hands_CS_34_Idle" true)))

(event Input|KeyboardEvents|8
  (params (Key :type Key%20Structure))
  (bind _hands (Variables|Default|GetHands))
  ;[1 1 1] Weapon Inspect
  (:Pressed
    (Components|Animation|PlayAnimation _hands "/Game/FPS/Weapons/SubmachineGun/CS_34_Smg/Animations/Hand_Animations/AS_Hands_CS_34_WeaponInspect.AS_Hands_CS_34_WeaponInspect" false)
    (Utilities|FlowControl|Delay 7.0)
    (Components|Animation|PlayAnimation _hands "/Game/FPS/Weapons/SubmachineGun/CS_34_Smg/Animations/Hand_Animations/AS_Hands_CS_34_Idle.AS_Hands_CS_34_Idle" true)))

(event Input|KeyboardEvents|1
  (params (Key :type Key%20Structure))
  ;[1 1 1] Weapon Equip
  (:Pressed
    (if (Variables|Default|GetWeapon%20is%20Spawned)
      _
      (else
        (Variables|Default|SetWeapon%20is%20Spawned true)
        (bind _returnvalue (Game|SpawnActorfromClass "/Game/FPS/Weapons/SubmachineGun/CS_34_Smg/Blueprints/BP_CS_34_SMG.BP_CS_34_SMG_C" (Transformation|GetSocketTransform (Variables|Default|GetHands) "cc_ItemHolder_rSocket" "RTS_World") "DontSpawnIfColliding" 0 0))
        (Transformation|AttachComponentToComponent _returnvalue (Variables|Default|GetHands) "cc_ItemHolder_rSocket" "SnapToTarget" "SnapToTarget" "SnapToTarget" true)
        (bind _outactors (Actor|GetAllActorsOfClass "/Game/FPS/Weapons/SubmachineGun/CS_34_Smg/Blueprints/BP_CS_34_SMG.BP_CS_34_SMG_C"))
        (Input|DisableInput (Utilities|Array|Get(acopy) _outactors) 0)))
    (Components|Animation|PlayAnimation (Variables|Default|GetHands) "/Game/FPS/Weapons/SubmachineGun/CS_34_Smg/Animations/Hand_Animations/AS_Hands_CS_34_Equip.AS_Hands_CS_34_Equip" false)
    (bind _outactors_2 (Actor|GetAllActorsOfClass "/Game/FPS/Weapons/SubmachineGun/CS_34_Smg/Blueprints/BP_CS_34_SMG.BP_CS_34_SMG_C"))
    (Default|HandsEquip (Utilities|Array|Get(acopy) _outactors_2))
    (Utilities|FlowControl|Delay 1.5)
    (Components|Animation|PlayAnimation (Variables|Default|GetHands) "/Game/FPS/Weapons/SubmachineGun/CS_34_Smg/Animations/Hand_Animations/AS_Hands_CS_34_Idle.AS_Hands_CS_34_Idle" true)))

(event Input|KeyboardEvents|2
  (params (Key :type Key%20Structure))
  (bind _hands (Variables|Default|GetHands))
  ;[1 1 1] Walking
  (:Pressed
    (Components|Animation|PlayAnimation _hands "/Game/FPS/Weapons/SubmachineGun/CS_34_Smg/Animations/Hand_Animations/AS_Hands_CS_34_Walking.AS_Hands_CS_34_Walking" true))
  (:Released
    (Components|Animation|PlayAnimation _hands "/Game/FPS/Weapons/SubmachineGun/CS_34_Smg/Animations/Hand_Animations/AS_Hands_CS_34_Idle.AS_Hands_CS_34_Idle" true)))

(fn ConstructionScript)