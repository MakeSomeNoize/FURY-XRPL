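; CS-34 submachine gun Blueprint that plays the weapon's equip, unequip, shoot, reload and full-reload animations.
; Number keys drive it standalone, while matching Hands events trigger the same logic and a separate event disables its input.
; Shots spawn used-bullet shells at the shell socket, with full-auto repeating on a short delay until release briefly clears a loop flag.
; Both reloads briefly hide the magazine ammo component.
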(event Custom|Disable%20input%20for%20weapon
  ;[1 1 1] Disabling imput when hands are holding weapon
  (Input|DisableInput 0))

(event Custom|Hands%20Sooting
  ;[1 1 1] Single Shoot
  (Components|Animation|PlayAnimation (Variables|Default|GetCS_34_SMG) "/Game/FPS/Weapons/SubmachineGun/CS_34_Smg/Animations/CS_34_SMG_Animations/AS_Weapon_CS_34_Shoot.AS_Weapon_CS_34_Shoot" false)
  ;[1 1 1] Shell Ejector
  (Game|SpawnActorfromClass "/Game/FPS/Weapons/SubmachineGun/CS_34_Smg/Blueprints/BP_Bullet_Used.BP_Bullet_Used_C" (Transformation|GetWorldTransform (Variables|Default|GetShell_Socket)) "AdjustIfPossibleButDontSpawnIfColliding" 0 0)
  (Utilities|FlowControl|Delay 0.08)
  (if (Variables|Default|GetLoopEnd)
    _))

(event Custom|Hands%20FullAutoShoot
  ;[1 1 1] Full_Auto_Shoot
  (Components|Animation|PlayAnimation (Variables|Default|GetCS_34_SMG) "/Game/FPS/Weapons/SubmachineGun/CS_34_Smg/Animations/CS_34_SMG_Animations/AS_Weapon_CS_34_Shoot.AS_Weapon_CS_34_Shoot" false :!label _label)
  ;[1 1 1] Shell Ejector
  (Game|SpawnActorfromClass "/Game/FPS/Weapons/SubmachineGun/CS_34_Smg/Blueprints/BP_Bullet_Used.BP_Bullet_Used_C" (Transformation|GetWorldTransform (Variables|Default|GetShell_Socket)) "Undefined" 0 0)
  (Utilities|FlowControl|Delay 0.08)
  (if (Variables|Default|GetLoopEnd)
    (goto _label)))

(event Custom|Hands%20Equip
  ;[1 1 1] Equip
  (Components|Animation|PlayAnimation (Variables|Default|GetCS_34_SMG) "/Game/FPS/Weapons/SubmachineGun/CS_34_Smg/Animations/CS_34_SMG_Animations/AS_Weapon_CS_34_Equip.AS_Weapon_CS_34_Equip" false) ; Animation with Hands USED
)

(event Custom|Hands%20full%20reload
  ;[1 1 1] fullreload
  (Components|Animation|PlayAnimation (Variables|Default|GetCS_34_SMG) "/Game/FPS/Weapons/SubmachineGun/CS_34_Smg/Animations/CS_34_SMG_Animations/AS_Weapon_CS_34_FullReload.AS_Weapon_CS_34_FullReload" false)
  (Rendering|SetVisibility (Variables|Default|GetAmmo_In_Magazine) false false)
  (Utilities|FlowControl|Delay 1.0)
  (Rendering|SetVisibility (Variables|Default|GetAmmo_In_Magazine) true false))

(event Custom|Hands%20Reloading
  ;[1 1 1] Reload
  (Components|Animation|PlayAnimation (Variables|Default|GetCS_34_SMG) "/Game/FPS/Weapons/SubmachineGun/CS_34_Smg/Animations/CS_34_SMG_Animations/AS_Weapon_CS_34_Reload.AS_Weapon_CS_34_Reload" false)
  (Rendering|SetVisibility (Variables|Default|GetAmmo_In_Magazine) false false)
  (Utilities|FlowControl|Delay 1.0)
  (Rendering|SetVisibility (Variables|Default|GetAmmo_In_Magazine) true false))

(event Custom|Hands%20Unequip
  ;[1 1 1] Unequip
  (Components|Animation|PlayAnimation (Variables|Default|GetCS_34_SMG) "/Game/FPS/Weapons/SubmachineGun/CS_34_Smg/Animations/CS_34_SMG_Animations/AS_Weapon_CS_34_UnEquip.AS_Weapon_CS_34_UnEquip" false) ; Animation With Hands USED
)

(event Custom|Hands%20Stop%20Full%20Auto%20Shooting
  ;[1 1 1] Full_Auto_Shoot
  (Variables|Default|SetLoopEnd false)
  (Utilities|FlowControl|Delay 0.1)
  (Variables|Default|SetLoopEnd true))

(event EventBeginPlay
  ;[1 1 1] Player Input
  (Input|EnableInput (Game|GetPlayerController 0)))

(event Input|KeyboardEvents|5
  (params (Key :type Key%20Structure :default "None"))
  ;[1 1 1] Reload
  (:Pressed
    (Components|Animation|PlayAnimation (Variables|Default|GetCS_34_SMG) "/Game/FPS/Weapons/SubmachineGun/CS_34_Smg/Animations/CS_34_SMG_Animations/AS_Weapon_CS_34_Reload.AS_Weapon_CS_34_Reload" false)
    (Rendering|SetVisibility (Variables|Default|GetAmmo_In_Magazine) false false)
    (Utilities|FlowControl|Delay 1.0)
    (Rendering|SetVisibility (Variables|Default|GetAmmo_In_Magazine) true false)))

(event Input|KeyboardEvents|2
  (params (Key :type Key%20Structure :default "None"))
  ;[1 1 1] Equip
  (:Pressed
    (Components|Animation|PlayAnimation (Variables|Default|GetCS_34_SMG) "/Game/FPS/Weapons/SubmachineGun/CS_34_Smg/Animations/CS_34_SMG_Animations/AS_Weapon_CS_34_Equip.AS_Weapon_CS_34_Equip" false) ; Animation with Hands USED
  ))

(event Input|KeyboardEvents|3
  (params (Key :type Key%20Structure :default "None"))
  ;[1 1 1] Single Shoot
  (:Pressed
    (Components|Animation|PlayAnimation (Variables|Default|GetCS_34_SMG) "/Game/FPS/Weapons/SubmachineGun/CS_34_Smg/Animations/CS_34_SMG_Animations/AS_Weapon_CS_34_Shoot.AS_Weapon_CS_34_Shoot" false)
    ;[1 1 1] Shell Ejector
    (Game|SpawnActorfromClass "/Game/FPS/Weapons/SubmachineGun/CS_34_Smg/Blueprints/BP_Bullet_Used.BP_Bullet_Used_C" (Transformation|GetWorldTransform (Variables|Default|GetShell_Socket)) "AdjustIfPossibleButDontSpawnIfColliding" 0 0)
    (Utilities|FlowControl|Delay 0.08)
    (if (Variables|Default|GetLoopEnd)
      _)))

(event Input|KeyboardEvents|4
  (params (Key :type Key%20Structure :default "None"))
  ;[1 1 1] Full_Auto_Shoot
  (:Pressed
    (Components|Animation|PlayAnimation (Variables|Default|GetCS_34_SMG) "/Game/FPS/Weapons/SubmachineGun/CS_34_Smg/Animations/CS_34_SMG_Animations/AS_Weapon_CS_34_Shoot.AS_Weapon_CS_34_Shoot" false :!label _label)
    ;[1 1 1] Shell Ejector
    (Game|SpawnActorfromClass "/Game/FPS/Weapons/SubmachineGun/CS_34_Smg/Blueprints/BP_Bullet_Used.BP_Bullet_Used_C" (Transformation|GetWorldTransform (Variables|Default|GetShell_Socket)) "Undefined" 0 0)
    (Utilities|FlowControl|Delay 0.08)
    (if (Variables|Default|GetLoopEnd)
      (goto _label)))
  (:Released
    (Variables|Default|SetLoopEnd false)
    (Utilities|FlowControl|Delay 0.1)
    (Variables|Default|SetLoopEnd true)))

(event Input|KeyboardEvents|1
  (params (Key :type Key%20Structure :default "None"))
  ;[1 1 1] Unequip
  (:Pressed
    (Components|Animation|PlayAnimation (Variables|Default|GetCS_34_SMG) "/Game/FPS/Weapons/SubmachineGun/CS_34_Smg/Animations/CS_34_SMG_Animations/AS_Weapon_CS_34_UnEquip.AS_Weapon_CS_34_UnEquip" false) ; Animation With Hands USED
  ))

(event Input|KeyboardEvents|6
  (params (Key :type Key%20Structure :default "None"))
  ;[1 1 1] fullreload
  (:Pressed
    (Components|Animation|PlayAnimation (Variables|Default|GetCS_34_SMG) "/Game/FPS/Weapons/SubmachineGun/CS_34_Smg/Animations/CS_34_SMG_Animations/AS_Weapon_CS_34_FullReload.AS_Weapon_CS_34_FullReload" false)
    (Rendering|SetVisibility (Variables|Default|GetAmmo_In_Magazine) false false)
    (Utilities|FlowControl|Delay 1.0)
    (Rendering|SetVisibility (Variables|Default|GetAmmo_In_Magazine) true false)))

(fn ConstructionScript)