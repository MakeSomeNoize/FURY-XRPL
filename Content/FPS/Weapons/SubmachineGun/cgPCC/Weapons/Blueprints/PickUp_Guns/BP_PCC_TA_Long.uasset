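; Child weapon Blueprint for the long PCC TA submachine gun pickup, handling its attachment visuals, muzzle smoke and magazine meshes.
; Construction snaps flashlight, spotlight and laser parts onto handguard sockets.
; Events swap iron sights for the scope, toggle rail parts with the flashlight, switch magazine meshes, and offset smoke when silenced.
; Tick updates the laser point only while this is the current weapon with a visible flashlight.
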(event EventScopeAttached
  ;[1 1 1] Scope Attached
  (CallFunction|IronSightStates))

(event EventFlashlightAttached
  ;[1 1 1] FlashlightAttached
  (CallFunction|PicRailVisibility))

(event EventMag02Vis
  ;[1 1 1] Magazine visibility
  (Rendering|SetVisibility (Variables|Default|GetSM_Magazine_02) true false))

(event EventMag02Invis
  ;[1 1 1] Magazine visibility
  (Rendering|SetVisibility (Variables|Default|GetSM_Magazine_02) false false))

(event EventMagVisible
  ;[1 1 1] Magazine visibility
  (if (Variables|Default|GetAutoReload?)
    (Rendering|SetVisibility (Variables|Default|GetSM_Magazine_Empty) true false)
    (Rendering|SetVisibility (Variables|Default|GetSM_Magazine_01) false false)
    (Rendering|SetVisibility (Variables|Default|GetSM_Magazine_02) false false)
    (else
      (Rendering|SetVisibility (Variables|Default|GetSM_Magazine_Empty) false false)
      (Rendering|SetVisibility (Variables|Default|GetSM_Magazine_01) true false)
      (Rendering|SetVisibility (Variables|Default|GetSM_Magazine_02) false false))))

(event EventBeginPlay
  (|CallParentFunction) ; This node is disabled and will not be called.\nDrag off pins to build functionality.
)

(event EventMagEmptyInvis
  ;[1 1 1] Magazine visibility
  (Rendering|SetVisibility (Variables|Default|GetSM_Magazine_Empty) false false))

(event EventMag01Visible
  ;[1 1 1] Magazine visibility
  (Rendering|SetVisibility (Variables|Default|GetSM_Magazine_01) true false))

(event EventMagEmptyVis
  ;[1 1 1] Magazine visibility
  (Rendering|SetVisibility (Variables|Default|GetSM_Magazine_Empty) true false))

(event EventBSmokeStop
  ;[1 1 1] MuzzleSmoke
  (Components|Activation|Deactivate (Variables|Default|GetMuzzleSmoke_PS))
  (Transformation|SetRelativeLocation (Variables|Default|GetMuzzleSmoke_PS) "0, 0, 0" false false))

(event EventBSmokeStart
  ;[1 1 1] MuzzleSmoke
  (if (> (.AmmoCurrent (Utilities|Struct|BreakBP_WeaponData_Struct (Variables|Default|GetWeaponData))) 0)
    (Utilities|FlowControl|Sequence
      (:then_0
        _)
      (:then_1
        (goto _label Reset)))
    (else
      (Utilities|FlowControl|DoOnce false :!label _label
        (:Completed
          _))))
  (Components|Activation|Activate (Variables|Default|GetMuzzleSmoke_PS) false)
  (if (Rendering|IsVisible (Variables|Default|GetSM_Silencer))
    (Transformation|SetRelativeLocation (Variables|Default|GetMuzzleSmoke_PS) (+ (Variables|/Script/Engine.SceneComponent|GetRelativeLocation (Variables|Default|GetMuzzleSmoke_PS)) "20.000000, 0, 0") false false)
    (else
      (Transformation|SetRelativeLocation (Variables|Default|GetMuzzleSmoke_PS) "0, 0, 0" false false))))

(event EventMAg01Invis
  ;[1 1 1] Magazine visibility
  (Rendering|SetVisibility (Variables|Default|GetSM_Magazine_01) false false))

(event EventTick
  (params (DeltaSeconds :type Float%20%28single-precision%29))
  ;[1 1 1] Laser
  (if (not (and (== self (Variables|/Game/cgPCC/FPS_Arms/Bluprints/BP_FPS_Arms.BP_FPS_Arms_C|GetCurrentWeapon (Variables|Default|GetCharacter%20Ref))) (Rendering|IsVisible (Variables|Default|GetSM_Flashlight))))
    (Rendering|SetVisibility (Variables|Default|GetSM_Laser) false false)
    (Rendering|SetVisibility (Variables|Default|GetLaser_Point) false false)
    (else
      (CallFunction|LaserPointPosition))))

(fn ConstructionScript
  (|CallParentFunction)
  (CallFunction|AttachtoComponentFunc))

(fn AttachtoComponentFunc
  (Transformation|AttachComponentToComponent (Variables|Default|GetSM_Flashlight) (Variables|Default|GetHandguard) "PWQ_Laser_Sckt" "SnapToTarget" "SnapToTarget" "SnapToTarget" true)
  (Transformation|AttachComponentToComponent (Variables|Default|GetSpotLight) (Variables|Default|GetSM_Flashlight) "Light_Sckt" "SnapToTarget" "SnapToTarget" "SnapToTarget" true)
  (Transformation|AttachComponentToComponent (Variables|Default|GetLaser_Point) (Variables|Default|GetSM_Flashlight) "Light_Sckt" "SnapToTarget" "SnapToTarget" "SnapToTarget" true)
  (Transformation|AttachComponentToComponent (Variables|Default|GetSM_Laser) (Variables|Default|GetSM_Flashlight) "Laser_Sckt" "SnapToTarget" "SnapToTarget" "SnapToTarget" true)
  (Transformation|SetRelativeScale3D (Variables|Default|GetSM_Laser) "10.000000,0.200000,0.200000"))

(fn IronSightStates
  (bind _irs_pro_front_raised (Variables|Default|GetIRS_pro_Front_Raised))
  (bind _irs_pro_front (Variables|Default|GetIRS_pro_Front))
  (if (Rendering|IsVisible (Variables|Default|GetSM_Scope))
    (Rendering|SetVisibility _irs_pro_front_raised false false)
    (Rendering|SetVisibility _irs_pro_front true false)
    (else
      (Rendering|SetVisibility _irs_pro_front_raised true false)
      (Rendering|SetVisibility _irs_pro_front false false))))

(fn PicRailVisibility
  (bind _picrail_l (Variables|Default|GetPicRail_L))
  (if (Rendering|IsVisible (Variables|Default|GetSM_Flashlight))
    (Rendering|SetVisibility _picrail_l true false)
    (else
      (Rendering|SetVisibility _picrail_l false false))))