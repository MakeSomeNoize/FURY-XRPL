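; Heat 772 assault rifle actor that plays weapon animations and doubles as an interactable pickup.
; Number keys or Hands events drive shooting, reloads and inspection (event only), toggling magazine meshes to match; input can be disabled when held.
; Shots spawn shell actors at ShellSocket; full auto repeats on a short delay until release briefly clears LoopEnd.
; Interact sends the pawn a BP_AssaultRifle pickup message with ammo, then destroys the actor.
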(event Custom|Disable%20input%20for%20weapon
  ;[1 1 1] Disabling imput when hands are holding weapon
  (Input|DisableInput 0))

(event Custom|Hands%20Shooting
  ;[1 1 1] Single Shoot
  (Components|Animation|PlayAnimation (Variables|Default|GetHeat_772) "/Game/FPS/Weapons/AssaultRifle/Heat_772_Rifle/Animations/Heat_772_Animations/AS_Weapon_Heat_772_Shooting.AS_Weapon_Heat_772_Shooting" false)
  ;[1 1 1] Shell Ejector
  (Game|SpawnActorfromClass "/Game/FPS/Blueprints/Bullets/OLD/BP_Bullet_Shell_Base_WithProjectile.BP_Bullet_Shell_Base_WithProjectile_C" (Transformation|GetWorldTransform (Variables|Default|GetShell_Socket)) "Undefined" 0 0)
  (Utilities|FlowControl|Delay 0.06)
  (if (Variables|Default|GetLoopEnd)
    _))

(event Custom|Hands%20Reloading
  ;[1 1 1] Reload
  (Components|Animation|PlayAnimation (Variables|Default|GetHeat_772) "/Game/FPS/Weapons/AssaultRifle/Heat_772_Rifle/Animations/Heat_772_Animations/AS_Weapon_Heat_772_Reload.AS_Weapon_Heat_772_Reload" false)
  (Rendering|SetVisibility (Variables|Default|GetAmmo_In_Magazine) false false)
  (Rendering|SetVisibility (Variables|Default|GetMagazine_2) true true)
  (Utilities|FlowControl|Delay 1.66666)
  (Rendering|SetVisibility (Variables|Default|GetAmmo_In_Magazine) false false)
  (Rendering|SetVisibility (Variables|Default|GetMagazine) false true))

(event Custom|Hands%20WeaponInspect
  ;[1 1 1] Weapon Inspecting
  (Components|Animation|PlayAnimation (Variables|Default|GetHeat_772) "/Game/FPS/Weapons/AssaultRifle/Heat_772_Rifle/Animations/Heat_772_Animations/AS_Weapon_Heat_772_WeaponInspect.AS_Weapon_Heat_772_WeaponInspect" false)
  (Rendering|SetVisibility (Variables|Default|GetAmmo_In_Magazine) true false)
  (Rendering|SetVisibility (Variables|Default|GetMagazine_2) false true))

(event Custom|Hands%20FullAutoShoot
  ;[1 1 1] Full_Auto_Shoot
  (Components|Animation|PlayAnimation (Variables|Default|GetHeat_772) "/Game/FPS/Weapons/AssaultRifle/Heat_772_Rifle/Animations/Heat_772_Animations/AS_Weapon_Heat_772_Shooting.AS_Weapon_Heat_772_Shooting" false :!label _label)
  ;[1 1 1] Shell Ejector
  (Game|SpawnActorfromClass "/Game/FPS/Blueprints/Bullets/OLD/BP_Bullet_Shell_Base_WithProjectile.BP_Bullet_Shell_Base_WithProjectile_C" (Transformation|GetWorldTransform (Variables|Default|GetShell_Socket)) "Undefined" 0 0)
  (Utilities|FlowControl|Delay 0.06)
  (if (Variables|Default|GetLoopEnd)
    (goto _label)))

(event Custom|Hands%20Full%20Reload
  ;[1 1 1] FullReload
  (Components|Animation|PlayAnimation (Variables|Default|GetHeat_772) "/Game/FPS/Weapons/AssaultRifle/Heat_772_Rifle/Animations/Heat_772_Animations/AS_Weapon_Heat_772_FullReload.AS_Weapon_Heat_772_FullReload" false)
  (Rendering|SetVisibility (Variables|Default|GetAmmo_In_Magazine) false false)
  (Rendering|SetVisibility (Variables|Default|GetMagazine_2) true true)
  (Utilities|FlowControl|Delay 2.53333)
  (Rendering|SetVisibility (Variables|Default|GetAmmo_In_Magazine) false false)
  (Rendering|SetVisibility (Variables|Default|GetMagazine) false true))

(event Custom|Hands%20Stop%20Full%20Auto%20Shooting
  ;[1 1 1] Full_Auto_Shoot
  (Variables|Default|SetLoopEnd false)
  (Utilities|FlowControl|Delay 0.1)
  (Variables|Default|SetLoopEnd true))

(event EventInteract
  (params (InstigatorPawn :type Pawn%20Object%20Reference))
  (Class|IPawnActions|OnPickupWeapon(Message) InstigatorPawn "/Game/FPS/Blueprints/Weapons/BP_AssaultRifle.BP_AssaultRifle_C" 11)
  (Actor|DestroyActor))

(event EventOnReset
  ;[0 0 0] On Reset
  (Actor|DestroyActor))

(event Input|KeyboardEvents|1
  (params (Key :type Key%20Structure))
  ;[1 1 1] Single Shoot
  (:Pressed
    (Components|Animation|PlayAnimation (Variables|Default|GetHeat_772) "/Game/FPS/Weapons/AssaultRifle/Heat_772_Rifle/Animations/Heat_772_Animations/AS_Weapon_Heat_772_Shooting.AS_Weapon_Heat_772_Shooting" false)
    ;[1 1 1] Shell Ejector
    (Game|SpawnActorfromClass "/Game/FPS/Blueprints/Bullets/OLD/BP_Bullet_Shell_Base_WithProjectile.BP_Bullet_Shell_Base_WithProjectile_C" (Transformation|GetWorldTransform (Variables|Default|GetShell_Socket)) "Undefined" 0 0)
    (Utilities|FlowControl|Delay 0.06)
    (if (Variables|Default|GetLoopEnd)
      _)))

(event Input|KeyboardEvents|3
  (params (Key :type Key%20Structure))
  ;[1 1 1] Full_Auto_Shoot
  (:Pressed
    (Components|Animation|PlayAnimation (Variables|Default|GetHeat_772) "/Game/FPS/Weapons/AssaultRifle/Heat_772_Rifle/Animations/Heat_772_Animations/AS_Weapon_Heat_772_Shooting.AS_Weapon_Heat_772_Shooting" false :!label _label)
    ;[1 1 1] Shell Ejector
    (Game|SpawnActorfromClass "/Game/FPS/Blueprints/Bullets/OLD/BP_Bullet_Shell_Base_WithProjectile.BP_Bullet_Shell_Base_WithProjectile_C" (Transformation|GetWorldTransform (Variables|Default|GetShell_Socket)) "Undefined" 0 0)
    (Utilities|FlowControl|Delay 0.06)
    (if (Variables|Default|GetLoopEnd)
      (goto _label)))
  (:Released
    (Variables|Default|SetLoopEnd false)
    (Utilities|FlowControl|Delay 0.1)
    (Variables|Default|SetLoopEnd true)))

(event Input|KeyboardEvents|2
  (params (Key :type Key%20Structure))
  ;[1 1 1] Reload
  (:Pressed
    (Components|Animation|PlayAnimation (Variables|Default|GetHeat_772) "/Game/FPS/Weapons/AssaultRifle/Heat_772_Rifle/Animations/Heat_772_Animations/AS_Weapon_Heat_772_Reload.AS_Weapon_Heat_772_Reload" false)
    (Rendering|SetVisibility (Variables|Default|GetAmmo_In_Magazine) false false)
    (Rendering|SetVisibility (Variables|Default|GetMagazine_2) true true)
    (Utilities|FlowControl|Delay 1.66666)
    (Rendering|SetVisibility (Variables|Default|GetAmmo_In_Magazine) false false)
    (Rendering|SetVisibility (Variables|Default|GetMagazine) false true)))

(event Input|KeyboardEvents|4
  (params (Key :type Key%20Structure))
  ;[1 1 1] FullReload
  (:Pressed
    (Components|Animation|PlayAnimation (Variables|Default|GetHeat_772) "/Game/FPS/Weapons/AssaultRifle/Heat_772_Rifle/Animations/Heat_772_Animations/AS_Weapon_Heat_772_FullReload.AS_Weapon_Heat_772_FullReload" false)
    (Rendering|SetVisibility (Variables|Default|GetAmmo_In_Magazine) false false)
    (Rendering|SetVisibility (Variables|Default|GetMagazine_2) true true)
    (Utilities|FlowControl|Delay 2.53333)
    (Rendering|SetVisibility (Variables|Default|GetAmmo_In_Magazine) false false)
    (Rendering|SetVisibility (Variables|Default|GetMagazine) false true)))

(fn ConstructionScript)

(fn GetDescription
  (return ""))

(fn GetIcon
  (return 0))

(fn GetInteractTime
  (return 0.5))

(fn TrytoInteract
  (return false))