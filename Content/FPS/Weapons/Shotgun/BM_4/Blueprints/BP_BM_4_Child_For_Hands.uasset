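; BP_BM_4_Child_For_Hands is a child Blueprint of the BM-4 shotgun, named for use in the player's hands, that plays the weapon's animations.
; Custom events play shot, silenced shot and reload animations on the skeletal mesh, with both shot events spawning an empty shell at the shell socket.
; Equipping the attachment plays a mount animation and briefly delays showing the barrel extender, which a separate event hides.
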(event Custom|BM4%20Reload
  ;[1 1 1] Reload
  (Components|Animation|PlayAnimation (Variables|Default|GetBM_4_Skeletal) "/Game/FPS/Weapons/Shotgun/BM_4/Animations/AS_BM_4_Load.AS_BM_4_Load" false))

(event Custom|scilencer%20shoot
  ;[1 1 1] Shoot
  (Components|Animation|PlayAnimation (Variables|Default|GetBM_4_Skeletal) "/Game/FPS/Weapons/Shotgun/BM_4/Animations/AS_BM_4_Shot_Extender.AS_BM_4_Shot_Extender" false)
  ;[1 1 1] Shell Ejector
  (Game|SpawnActorfromClass "/Game/FPS/Weapons/Shotgun/BM_4/Blueprints/BP_BM_4_Empty_Shell.BP_BM_4_Empty_Shell_C" (Transformation|GetWorldTransform (Variables|Default|GetShell_Socket)) "Undefined" 0 0))

(event Custom|Attachment%20hide
  ;[1 1 1] Extender Mount
  (Rendering|SetVisibility (Variables|Default|GetBM_4_Barrel_Extender) false false))

(event Custom|Equip%20Attachment
  ;[1 1 1] Extender Mount
  (Components|Animation|PlayAnimation (Variables|Default|GetBM_4_Skeletal) "/Game/FPS/Weapons/Shotgun/BM_4/Animations/AS_BM_4_Extender_Mount.AS_BM_4_Extender_Mount" false)
  (Utilities|FlowControl|Delay 0.1)
  (Rendering|SetVisibility (Variables|Default|GetBM_4_Barrel_Extender) true false))

(event Custom|BM4%20Shoot
  ;[1 1 1] Shoot
  (Components|Animation|PlayAnimation (Variables|Default|GetBM_4_Skeletal) "/Game/FPS/Weapons/Shotgun/BM_4/Animations/AS_BM_4_Shot.AS_BM_4_Shot" false)
  ;[1 1 1] Shell Ejector
  (Game|SpawnActorfromClass "/Game/FPS/Weapons/Shotgun/BM_4/Blueprints/BP_BM_4_Empty_Shell.BP_BM_4_Empty_Shell_C" (Transformation|GetWorldTransform (Variables|Default|GetShell_Socket)) "Undefined" 0 0))

(event EventBeginPlay
  ;[1 1 1] Player Input
  (Input|EnableInput (Game|GetPlayerController 0)))

(fn ConstructionScript
  (|CallParentFunction))