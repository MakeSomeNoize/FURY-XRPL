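; BP_BM_4 is a BM-4 shotgun actor that previews the weapon's animations through hard-wired number-key input from the first player controller.
; Each key plays a one-shot skeletal animation for reload, load, shot, shot with extender, or extender mount and removal.
; Both shot actions spawn an empty shell actor at the shell socket component's transform.
; Mount and removal toggle barrel extender visibility after short delays timed to their animations.
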(event EventBeginPlay
  ;[1 1 1] Player Input
  (Input|EnableInput (Game|GetPlayerController 0)))

(event Input|KeyboardEvents|5
  (params (Key :type Key%20Structure :default "None"))
  ;[1 1 1] Shoot_Extender
  (:Pressed
    (Components|Animation|PlayAnimation (Variables|Default|GetBM_4_Skeletal) "/Game/FPS/Weapons/Shotgun/BM_4/Animations/AS_BM_4_Shot_Extender.AS_BM_4_Shot_Extender" false)
    ;[1 1 1] Shell Ejector
    (Game|SpawnActorfromClass "/Game/FPS/Weapons/Shotgun/BM_4/Blueprints/BP_BM_4_Empty_Shell.BP_BM_4_Empty_Shell_C" (Transformation|GetWorldTransform (Variables|Default|GetShell_Socket)) "Undefined" 0 0)))

(event Input|KeyboardEvents|3
  (params (Key :type Key%20Structure :default "None"))
  ;[1 1 1] Shoot
  (:Pressed
    (Components|Animation|PlayAnimation (Variables|Default|GetBM_4_Skeletal) "/Game/FPS/Weapons/Shotgun/BM_4/Animations/AS_BM_4_Load.AS_BM_4_Load" false)))

(event Input|KeyboardEvents|6
  (params (Key :type Key%20Structure :default "None"))
  ;[1 1 1] Extender Mount
  (:Pressed
    (Components|Animation|PlayAnimation (Variables|Default|GetBM_4_Skeletal) "/Game/FPS/Weapons/Shotgun/BM_4/Animations/AS_BM_4_Extender_Remove.AS_BM_4_Extender_Remove" false)
    (Utilities|FlowControl|Delay 1.3)
    (Development|SetHiddeninGame (Variables|Default|GetBM_4_Barrel_Extender) true false)))

(event Input|KeyboardEvents|4
  (params (Key :type Key%20Structure :default "None"))
  ;[1 1 1] Extender Mount
  (:Pressed
    (Components|Animation|PlayAnimation (Variables|Default|GetBM_4_Skeletal) "/Game/FPS/Weapons/Shotgun/BM_4/Animations/AS_BM_4_Extender_Mount.AS_BM_4_Extender_Mount" false)
    (Utilities|FlowControl|Delay 0.1)
    (Development|SetHiddeninGame (Variables|Default|GetBM_4_Barrel_Extender) false false)))

(event Input|KeyboardEvents|1
  (params (Key :type Key%20Structure :default "None"))
  ;[1 1 1] Reload
  (:Pressed
    (Components|Animation|PlayAnimation (Variables|Default|GetBM_4_Skeletal) "/Game/FPS/Weapons/Shotgun/BM_4/Animations/AS_BM_4_Reload.AS_BM_4_Reload" false)))

(event Input|KeyboardEvents|2
  (params (Key :type Key%20Structure :default "None"))
  ;[1 1 1] Shoot
  (:Pressed
    (Components|Animation|PlayAnimation (Variables|Default|GetBM_4_Skeletal) "/Game/FPS/Weapons/Shotgun/BM_4/Animations/AS_BM_4_Shot.AS_BM_4_Shot" false)
    ;[1 1 1] Shell Ejector
    (Game|SpawnActorfromClass "/Game/FPS/Weapons/Shotgun/BM_4/Blueprints/BP_BM_4_Empty_Shell.BP_BM_4_Empty_Shell_C" (Transformation|GetWorldTransform (Variables|Default|GetShell_Socket)) "Undefined" 0 0)))

(fn ConstructionScript)