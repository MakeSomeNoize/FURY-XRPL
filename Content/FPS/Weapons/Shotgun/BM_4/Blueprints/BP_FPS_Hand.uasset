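; First-person hands actor that previews the BM-4 shotgun animation set through hard-coded keyboard keys.
; The equip key spawns the weapon actor once, attaches it to the Hands socket, disables its input and hides attachments.
; Keys play hand animations directly, with Delays returning some to idle.
; Reload, shoot, silenced shot and attachment equip also call the weapon, found via GetAllActorsOfClass rather than a stored reference.
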(event EventBeginPlay
  ;[1 1 1] Player Input
  (Input|EnableInput (Game|GetPlayerController 0)))

(event Input|KeyboardEvents|5
  (params (Key :type Key%20Structure :default "None"))
  ;[1 1 1] Reload
  (:Pressed
    (if (Variables|Default|GetWeapon%20is%20Spawned)
      (bind _outactors (Actor|GetAllActorsOfClass "/Game/FPS/Weapons/Shotgun/BM_4/Blueprints/BP_BM_4_Child_For_Hands.BP_BM_4_Child_For_Hands_C"))
      (Default|BM4Reload (Utilities|Array|Get(acopy) _outactors)))
    (Components|Animation|PlayAnimation (Variables|Default|GetHands) "/Game/FPS/Weapons/Shotgun/BM_4/Animations/Hand_Anims/AS_Hands_BM_4_Reload.AS_Hands_BM_4_Reload" false)
    (Utilities|FlowControl|Delay 0.8)
    (Components|Animation|PlayAnimation (Variables|Default|GetHands) "/Game/FPS/Weapons/Shotgun/BM_4/Animations/Hand_Anims/AS_Hands_BM_4_Idle.AS_Hands_BM_4_Idle" false)))

(event Input|KeyboardEvents|4
  (params (Key :type Key%20Structure :default "None"))
  ;[1 1 1] Shooting
  (:Pressed
    (if (Variables|Default|GetWeapon%20is%20Spawned)
      (bind _outactors (Actor|GetAllActorsOfClass "/Game/FPS/Weapons/Shotgun/BM_4/Blueprints/BP_BM_4_Child_For_Hands.BP_BM_4_Child_For_Hands_C"))
      (Default|BM4Shoot (Utilities|Array|Get(acopy) _outactors)))
    (Components|Animation|PlayAnimation (Variables|Default|GetHands) "/Game/FPS/Weapons/Shotgun/BM_4/Animations/Hand_Anims/AS_Hands_BM_4_Shoot.AS_Hands_BM_4_Shoot" false)))

(event Input|KeyboardEvents|0
  (params (Key :type Key%20Structure :default "None"))
  (bind _hands (Variables|Default|GetHands))
  ;[1 1 1] Scope UnAim
  (:Pressed
    (Components|Animation|PlayAnimation _hands "/Game/FPS/Weapons/Shotgun/BM_4/Animations/Hand_Anims/AS_Hands_BM_4_UnAim.AS_Hands_BM_4_UnAim" false)
    (Utilities|FlowControl|Delay 0.427)
    (Components|Animation|PlayAnimation _hands "/Game/FPS/Weapons/Shotgun/BM_4/Animations/Hand_Anims/AS_Hands_BM_4_Idle.AS_Hands_BM_4_Idle" true)))

(event Input|KeyboardEvents|Hyphen
  (params (Key :type Key%20Structure :default "None"))
  ;[1 1 1] Weapon unequip
  (:Pressed
    (if (Variables|Default|GetWeapon%20is%20Spawned)
      (Components|Animation|PlayAnimation (Variables|Default|GetHands) "/Game/FPS/Weapons/Shotgun/BM_4/Animations/Hand_Anims/AS_Hands_BM_4_UnEquip.AS_Hands_BM_4_UnEquip" false))))

(event Input|KeyboardEvents|8
  (params (Key :type Key%20Structure :default "None"))
  ;[1 1 1] Scope Aim
  (:Pressed
    (Components|Animation|PlayAnimation (Variables|Default|GetHands) "/Game/FPS/Weapons/Shotgun/BM_4/Animations/Hand_Anims/AS_Hands_BM_4_Aim.AS_Hands_BM_4_Aim" false)))

(event Input|KeyboardEvents|3
  (params (Key :type Key%20Structure :default "None"))
  (bind _hands (Variables|Default|GetHands))
  ;[1 1 1] Running
  (:Pressed
    (Components|Animation|PlayAnimation _hands "/Game/FPS/Weapons/Shotgun/BM_4/Animations/Hand_Anims/AS_Hands_BM_4_Running.AS_Hands_BM_4_Running" true))
  (:Released
    (Components|Animation|PlayAnimation _hands "/Game/FPS/Weapons/Shotgun/BM_4/Animations/Hand_Anims/AS_Hands_BM_4_Idle.AS_Hands_BM_4_Idle" true)))

(event Input|KeyboardEvents|9
  (params (Key :type Key%20Structure :default "None"))
  ;[1 1 1] Shooting
  (:Pressed
    (if (Variables|Default|GetWeapon%20is%20Spawned)
      (bind _outactors (Actor|GetAllActorsOfClass "/Game/FPS/Weapons/Shotgun/BM_4/Blueprints/BP_BM_4_Child_For_Hands.BP_BM_4_Child_For_Hands_C"))
      (Default|ScilencerShoot (Utilities|Array|Get(acopy) _outactors)))
    (Components|Animation|PlayAnimation (Variables|Default|GetHands) "/Game/FPS/Weapons/Shotgun/BM_4/Animations/Hand_Anims/AS_Hands_BM_4_Aim_Shoot.AS_Hands_BM_4_Aim_Shoot" false)))

(event Input|KeyboardEvents|6
  (params (Key :type Key%20Structure :default "None"))
  (bind _hands (Variables|Default|GetHands))
  ;[1 1 1] Attachmments Equip
  (:Pressed
    (bind _outactors (Actor|GetAllActorsOfClass "/Game/FPS/Weapons/Shotgun/BM_4/Blueprints/BP_BM_4_Child_For_Hands.BP_BM_4_Child_For_Hands_C"))
    (Default|EquipAttachment (Utilities|Array|Get(acopy) _outactors))
    (Components|Animation|PlayAnimation _hands "/Game/FPS/Weapons/Shotgun/BM_4/Animations/Hand_Anims/AS_Hands_BM_4_AttachmentsEquiping.AS_Hands_BM_4_AttachmentsEquiping" false)
    (Utilities|FlowControl|Delay 7.0)
    (Components|Animation|PlayAnimation _hands "/Game/FPS/Weapons/Shotgun/BM_4/Animations/Hand_Anims/AS_Hands_BM_4_Idle.AS_Hands_BM_4_Idle" true)))

(event Input|KeyboardEvents|1
  (params (Key :type Key%20Structure :default "None"))
  ;[1 1 1] Weapon Equip
  (:Pressed
    (if (Variables|Default|GetWeapon%20is%20Spawned)
      _
      (else
        (Variables|Default|SetWeapon%20is%20Spawned true)
        (bind _returnvalue (Game|SpawnActorfromClass "/Game/FPS/Weapons/Shotgun/BM_4/Blueprints/BP_BM_4_Child_For_Hands.BP_BM_4_Child_For_Hands_C" (Transformation|GetSocketTransform (Variables|Default|GetHands) "cc_ItemHolder_rSocket" "RTS_World") "DontSpawnIfColliding" 0 0))
        (Transformation|AttachComponentToComponent _returnvalue (Variables|Default|GetHands) "cc_ItemHolder_rSocket" "SnapToTarget" "SnapToTarget" "SnapToTarget" true)
        (bind _outactors (Actor|GetAllActorsOfClass "/Game/FPS/Weapons/Shotgun/BM_4/Blueprints/BP_BM_4_Child_For_Hands.BP_BM_4_Child_For_Hands_C"))
        (Input|DisableInput (Utilities|Array|Get(acopy) _outactors) 0)))
    (Components|Animation|PlayAnimation (Variables|Default|GetHands) "/Game/FPS/Weapons/Shotgun/BM_4/Animations/Hand_Anims/AS_Hands_BM_4_Equip.AS_Hands_BM_4_Equip" false)
    (Default|AttachmentHide (Utilities|Array|Get(acopy) _outactors))
    (Utilities|FlowControl|Delay 0.5)
    (Components|Animation|PlayAnimation (Variables|Default|GetHands) "/Game/FPS/Weapons/Shotgun/BM_4/Animations/Hand_Anims/AS_Hands_BM_4_Idle.AS_Hands_BM_4_Idle" true)))

(event Input|KeyboardEvents|7
  (params (Key :type Key%20Structure :default "None"))
  (bind _hands (Variables|Default|GetHands))
  ;[1 1 1] Weapon Inspect
  (:Pressed
    (Components|Animation|PlayAnimation _hands "/Game/FPS/Weapons/Shotgun/BM_4/Animations/Hand_Anims/AS_Hands_BM_4_WeaponInspect.AS_Hands_BM_4_WeaponInspect" false)
    (Utilities|FlowControl|Delay 7.0)
    (Components|Animation|PlayAnimation _hands "/Game/FPS/Weapons/Shotgun/BM_4/Animations/Hand_Anims/AS_Hands_BM_4_Idle.AS_Hands_BM_4_Idle" true)))

(event Input|KeyboardEvents|2
  (params (Key :type Key%20Structure :default "None"))
  (bind _hands (Variables|Default|GetHands))
  ;[1 1 1] Walking
  (:Pressed
    (Components|Animation|PlayAnimation _hands "/Game/FPS/Weapons/Shotgun/BM_4/Animations/Hand_Anims/AS_Hands_BM_4_Walking.AS_Hands_BM_4_Walking" true))
  (:Released
    (Components|Animation|PlayAnimation _hands "/Game/FPS/Weapons/Shotgun/BM_4/Animations/Hand_Anims/AS_Hands_BM_4_Idle.AS_Hands_BM_4_Idle" true)))

(fn ConstructionScript)