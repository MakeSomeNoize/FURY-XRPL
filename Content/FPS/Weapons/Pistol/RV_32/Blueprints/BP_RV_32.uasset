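; BP_RV_32 is the RV-32 pistol actor, which plays the weapon's equip, single-shot and reload animations.
; It enables player input at BeginPlay so keys 1–3 trigger those animations, with an event that disables input when hands hold the weapon.
; Hands-prefixed events jump into the same animation paths as the keys.
; Reload also shows the QuickLoader component, then hides it after a timed delay.
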(event Custom|Disable%20input%20for%20weapon
  ;[1 1 1] Disabling imput when hands are holding weapon
  (Input|DisableInput 0))

(event Custom|Hands%20Sooting
  ;[1 1 1] Single Shoot
  (Components|Animation|PlayAnimation (Variables|Default|GetRV_32) "/Game/FPS/Weapons/Pistol/RV_32/Animations/RV_32_Animations/AS_Weapon_RV_32_Shooting.AS_Weapon_RV_32_Shooting" false))

(event Custom|Hands%20Reloading
  ;[1 1 1] Reload
  (Components|Animation|PlayAnimation (Variables|Default|GetRV_32) "/Game/FPS/Weapons/Pistol/RV_32/Animations/RV_32_Animations/AS_Weapon_RV_32_Reload.AS_Weapon_RV_32_Reload" false)
  (Rendering|SetVisibility (Variables|Default|GetQuick_Loader) true false)
  (Utilities|FlowControl|Delay 1.11)
  (Rendering|SetVisibility (Variables|Default|GetQuick_Loader) false false))

(event Custom|Hands%20Equip
  ;[1 1 1] Equip
  (Components|Animation|PlayAnimation (Variables|Default|GetRV_32) "/Game/FPS/Weapons/Pistol/RV_32/Animations/RV_32_Animations/AS_Weapon_RV_32_Equip.AS_Weapon_RV_32_Equip" false))

(event EventBeginPlay
  ;[1 1 1] Player Input
  (Input|EnableInput (Game|GetPlayerController 0)))

(event Input|KeyboardEvents|3
  (params (Key :type Key%20Structure :default "None"))
  ;[1 1 1] Reload
  (:Pressed
    (Components|Animation|PlayAnimation (Variables|Default|GetRV_32) "/Game/FPS/Weapons/Pistol/RV_32/Animations/RV_32_Animations/AS_Weapon_RV_32_Reload.AS_Weapon_RV_32_Reload" false)
    (Rendering|SetVisibility (Variables|Default|GetQuick_Loader) true false)
    (Utilities|FlowControl|Delay 1.11)
    (Rendering|SetVisibility (Variables|Default|GetQuick_Loader) false false)))

(event Input|KeyboardEvents|2
  (params (Key :type Key%20Structure :default "None"))
  ;[1 1 1] Single Shoot
  (:Pressed
    (Components|Animation|PlayAnimation (Variables|Default|GetRV_32) "/Game/FPS/Weapons/Pistol/RV_32/Animations/RV_32_Animations/AS_Weapon_RV_32_Shooting.AS_Weapon_RV_32_Shooting" false)))

(event Input|KeyboardEvents|1
  (params (Key :type Key%20Structure :default "None"))
  ;[1 1 1] Equip
  (:Pressed
    (Components|Animation|PlayAnimation (Variables|Default|GetRV_32) "/Game/FPS/Weapons/Pistol/RV_32/Animations/RV_32_Animations/AS_Weapon_RV_32_Equip.AS_Weapon_RV_32_Equip" false)))

(fn ConstructionScript)