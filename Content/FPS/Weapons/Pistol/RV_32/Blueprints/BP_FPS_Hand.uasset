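; First-person hands actor that demos the RV-32 pistol animation set through number-key input.
; Key 1 spawns BP_RV_32 once and snaps it to the hands' item socket; other keys play equip, movement, aim, shoot, reload, inspect and unequip animations directly.
; Equip, shoot and reload also call matching events on the pistol, found via GetAllActorsOfClass.
; Fixed delays return most one-shot animations to idle.
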(event EventBeginPlay
  ;[1 1 1] Player Input
  (Input|EnableInput (Game|GetPlayerController 0)))

(event Input|KeyboardEvents|6
  (params (Key :type Key%20Structure))
  (bind _hands (Variables|Default|GetHands))
  ;[1 1 1] Weapon Inspect
  (:Pressed
    (Components|Animation|PlayAnimation _hands "/Game/FPS/Weapons/Pistol/RV_32/Animations/FPS_Hands_Animation/AS_Hands_RV_32_WeaponInspect.AS_Hands_RV_32_WeaponInspect" false)
    (Utilities|FlowControl|Delay 6.3)
    (Components|Animation|PlayAnimation _hands "/Game/FPS/Weapons/Pistol/RV_32/Animations/FPS_Hands_Animation/AS_Hands_RV_32_Idle.AS_Hands_RV_32_Idle" true)))

(event Input|KeyboardEvents|5
  (params (Key :type Key%20Structure))
  ;[1 1 1] Reload
  (:Pressed
    (if (Variables|Default|GetWeapon%20is%20Spawned)
      (bind _outactors (Actor|GetAllActorsOfClass "/Game/FPS/Weapons/Pistol/RV_32/Blueprints/BP_RV_32.BP_RV_32_C"))
      (Default|HandsReloading (Utilities|Array|Get(acopy) _outactors)))
    (Components|Animation|PlayAnimation (Variables|Default|GetHands) "/Game/FPS/Weapons/Pistol/RV_32/Animations/FPS_Hands_Animation/AS_Hands_RV_32_Reload.AS_Hands_RV_32_Reload" false)
    (Utilities|FlowControl|Delay 1.8)
    (Components|Animation|PlayAnimation (Variables|Default|GetHands) "/Game/FPS/Weapons/Pistol/RV_32/Animations/FPS_Hands_Animation/AS_Hands_RV_32_Idle.AS_Hands_RV_32_Idle" true)))

(event Input|KeyboardEvents|7
  (params (Key :type Key%20Structure))
  ;[1 1 1] Scope Aim
  (:Pressed
    (Components|Animation|PlayAnimation (Variables|Default|GetHands) "/Game/FPS/Weapons/Pistol/RV_32/Animations/FPS_Hands_Animation/AS_Hands_RV_32_Aim.AS_Hands_RV_32_Aim" false)))

(event Input|KeyboardEvents|8
  (params (Key :type Key%20Structure))
  ;[1 1 1] Shooting
  (:Pressed
    (if (Variables|Default|GetWeapon%20is%20Spawned)
      (bind _outactors (Actor|GetAllActorsOfClass "/Game/FPS/Weapons/Pistol/RV_32/Blueprints/BP_RV_32.BP_RV_32_C"))
      (Default|HandsSooting (Utilities|Array|Get(acopy) _outactors)))
    (Components|Animation|PlayAnimation (Variables|Default|GetHands) "/Game/FPS/Weapons/Pistol/RV_32/Animations/FPS_Hands_Animation/AS_Hands_RV_32_Aim_Shoot.AS_Hands_RV_32_Aim_Shoot" false)))

(event Input|KeyboardEvents|3
  (params (Key :type Key%20Structure))
  (bind _hands (Variables|Default|GetHands))
  ;[1 1 1] Running
  (:Pressed
    (Components|Animation|PlayAnimation _hands "/Game/FPS/Weapons/Pistol/RV_32/Animations/FPS_Hands_Animation/AS_Hands_RV_32_Running.AS_Hands_RV_32_Running" true))
  (:Released
    (Components|Animation|PlayAnimation _hands "/Game/FPS/Weapons/Pistol/RV_32/Animations/FPS_Hands_Animation/AS_Hands_RV_32_Idle.AS_Hands_RV_32_Idle" true)))

(event Input|KeyboardEvents|4
  (params (Key :type Key%20Structure))
  ;[1 1 1] Shooting
  (:Pressed
    (if (Variables|Default|GetWeapon%20is%20Spawned)
      (bind _outactors (Actor|GetAllActorsOfClass "/Game/FPS/Weapons/Pistol/RV_32/Blueprints/BP_RV_32.BP_RV_32_C"))
      (Default|HandsSooting (Utilities|Array|Get(acopy) _outactors)))
    (Components|Animation|PlayAnimation (Variables|Default|GetHands) "/Game/FPS/Weapons/Pistol/RV_32/Animations/FPS_Hands_Animation/AS_Hands_RV_32_Shooting.AS_Hands_RV_32_Shooting" false)
    (Utilities|FlowControl|Delay 0.27)
    (Components|Animation|PlayAnimation (Variables|Default|GetHands) "/Game/FPS/Weapons/Pistol/RV_32/Animations/FPS_Hands_Animation/AS_Hands_RV_32_Idle.AS_Hands_RV_32_Idle" false)))

(event Input|KeyboardEvents|9
  (params (Key :type Key%20Structure))
  (bind _hands (Variables|Default|GetHands))
  ;[1 1 1] Scope UnAim
  (:Pressed
    (Components|Animation|PlayAnimation _hands "/Game/FPS/Weapons/Pistol/RV_32/Animations/FPS_Hands_Animation/AS_Hands_RV_32_UnAim.AS_Hands_RV_32_UnAim" false)
    (Utilities|FlowControl|Delay 0.3)
    (Components|Animation|PlayAnimation _hands "/Game/FPS/Weapons/Pistol/RV_32/Animations/FPS_Hands_Animation/AS_Hands_RV_32_Idle.AS_Hands_RV_32_Idle" true)))

(event Input|KeyboardEvents|1
  (params (Key :type Key%20Structure))
  ;[1 1 1] Weapon Equip
  (:Pressed
    (if (Variables|Default|GetWeapon%20is%20Spawned)
      _
      (else
        (Variables|Default|SetWeapon%20is%20Spawned true)
        (bind _returnvalue (Game|SpawnActorfromClass "/Game/FPS/Weapons/Pistol/RV_32/Blueprints/BP_RV_32.BP_RV_32_C" (Transformation|GetSocketTransform (Variables|Default|GetHands) "cc_ItemHolder_rSocket" "RTS_World") "DontSpawnIfColliding" 0 0))
        (Transformation|AttachComponentToComponent _returnvalue (Variables|Default|GetHands) "cc_ItemHolder_rSocket" "SnapToTarget" "SnapToTarget" "SnapToTarget" true)
        (bind _outactors (Actor|GetAllActorsOfClass "/Game/FPS/Weapons/Pistol/RV_32/Blueprints/BP_RV_32.BP_RV_32_C"))
        (Input|DisableInput (Utilities|Array|Get(acopy) _outactors) 0)))
    (Components|Animation|PlayAnimation (Variables|Default|GetHands) "/Game/FPS/Weapons/Pistol/RV_32/Animations/FPS_Hands_Animation/AS_Hands_RV_32_Equip.AS_Hands_RV_32_Equip" false)
    (bind _outactors_2 (Actor|GetAllActorsOfClass "/Game/FPS/Weapons/Pistol/RV_32/Blueprints/BP_RV_32.BP_RV_32_C"))
    (Default|HandsEquip (Utilities|Array|Get(acopy) _outactors_2))
    (Utilities|FlowControl|Delay 0.8666)
    (Components|Animation|PlayAnimation (Variables|Default|GetHands) "/Game/FPS/Weapons/Pistol/RV_32/Animations/FPS_Hands_Animation/AS_Hands_RV_32_Idle.AS_Hands_RV_32_Idle" true)))

(event Input|KeyboardEvents|0
  (params (Key :type Key%20Structure))
  ;[1 1 1] Weapon unequip
  (:Pressed
    (Components|Animation|PlayAnimation (Variables|Default|GetHands) "/Game/FPS/Weapons/Pistol/RV_32/Animations/FPS_Hands_Animation/AS_Hands_RV_32_UnEqip.AS_Hands_RV_32_UnEqip" false)))

(event Input|KeyboardEvents|2
  (params (Key :type Key%20Structure))
  (bind _hands (Variables|Default|GetHands))
  ;[1 1 1] Walking
  (:Pressed
    (Components|Animation|PlayAnimation _hands "/Game/FPS/Weapons/Pistol/RV_32/Animations/FPS_Hands_Animation/AS_Hands_RV_32_Walking.AS_Hands_RV_32_Walking" true))
  (:Released
    (Components|Animation|PlayAnimation _hands "/Game/FPS/Weapons/Pistol/RV_32/Animations/FPS_Hands_Animation/AS_Hands_RV_32_Idle.AS_Hands_RV_32_Idle" true)))

(fn ConstructionScript)