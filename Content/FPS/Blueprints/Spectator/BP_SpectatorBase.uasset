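; Base spectator actor that gives the local player a spectator HUD and a route back to character selection.
; On becoming view target, it creates the widget, adds the spectator input context and enables spring-arm camera lag after a delay.
; Spawn input opens character selection if match settings allow respawn and the widget-assigned CanRespawn event has fired.
; Post-round and post-match events from AC_MatchStateSystem, or a reset, remove the widget and input context.
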(event Custom|CanRespawn
  ;[0 0 0] On BecomeViewTarget
  (Variables|Default|SetbCanRespawn true))

(event Custom|DestroyWidget
  (bind _wb_spectator (Variables|Default|GetWB_Spectator))
  ;[0 0 0] On BecomeViewTarget
  ;;[0 0 0] On Reset
  (Input|RemoveMappingContext (PlayerController|LocalPlayerSubsystems|GetEnhancedInputLocalPlayerSubsystem (Game|GetPlayerController 0)) "/Game/FPS/Inputs/IMC_SpectatorInputs.IMC_SpectatorInputs" "(bIgnoreAllPressedKeysUntilRelease=True,bForceImmediately=False)")
  (Utilities|IsValid _wb_spectator
    (:Is%20Valid
      (Widget|RemovefromParent _wb_spectator))))

(event Input|EnhancedActionEvents|EnhancedInputActionIA_Spawn
  (params (ActionValue :type Boolean) (ElapsedSeconds :type Float%20%28double-precision%29) (TriggeredSeconds :type Float%20%28double-precision%29) (InputAction :type Input%20Action%20Object%20Reference :default "/Game/FPS/Inputs/InputActions/IA_Spawn.IA_Spawn"))
  (bind _returnvalue (Game|GetGameState))
  (bind _returnvalue_2 (Actor|GetComponentbyClass _returnvalue "/Game/FPS/Blueprints/BlueprintsComponents/AC_MatchStateSystem.AC_MatchStateSystem_C"))
  ;[0 0 0] Show Character select
  (:Started
    (if (or (Default|IsGameOver _returnvalue_2) (Default|IsRoundOver _returnvalue_2))
      (Widget|RemovefromParent (Variables|Default|GetWB_Spectator))
      (elif (and (Default|GetAllowRespawn (Actor|GetComponentbyClass _returnvalue "/Game/FPS/Blueprints/BlueprintsComponents/AC_MatchSettings.AC_MatchSettings_C")) (Variables|Default|GetbCanRespawn))
        (Input|RemoveMappingContext (PlayerController|LocalPlayerSubsystems|GetEnhancedInputLocalPlayerSubsystem (Game|GetPlayerController 0)) "/Game/FPS/Inputs/IMC_SpectatorInputs.IMC_SpectatorInputs" "(bIgnoreAllPressedKeysUntilRelease=True,bForceImmediately=False)")
        (Default|ClientShowCharacterSelectionWidget (Actor|GetComponentbyClass (Game|GetPlayerController 0) "/Game/FPS/Blueprints/BlueprintsComponents/AC_UI_Manager.AC_UI_Manager_C"))
        (Widget|RemovefromParent (Variables|Default|GetWB_Spectator))))))

(event Input|EnhancedActionEvents|EnhancedInputActionIA_NextAlly
  (params (ActionValue :type Boolean) (ElapsedSeconds :type Float%20%28double-precision%29) (TriggeredSeconds :type Float%20%28double-precision%29) (InputAction :type Input%20Action%20Object%20Reference :default "/Game/FPS/Inputs/InputActions/IA_NextAlly.IA_NextAlly")))

(event EventOnReset
  (bind _wb_spectator (Variables|Default|GetWB_Spectator))
  ;[0 0 0] On BecomeViewTarget
  ;;[0 0 0] On Reset
  (Input|RemoveMappingContext (PlayerController|LocalPlayerSubsystems|GetEnhancedInputLocalPlayerSubsystem (Game|GetPlayerController 0)) "/Game/FPS/Inputs/IMC_SpectatorInputs.IMC_SpectatorInputs" "(bIgnoreAllPressedKeysUntilRelease=True,bForceImmediately=False)")
  (Utilities|IsValid _wb_spectator
    (:Is%20Valid
      (Widget|RemovefromParent _wb_spectator))))

(event EventOnBecomeViewTarget
  (params (PC :type Player%20Controller%20Object%20Reference))
  (bind _returnvalue (Game|GetGameState))
  (bind _returnvalue_2 (Game|GetPlayerController 0))
  (bind _returnvalue_3 (Actor|GetComponentbyClass _returnvalue "/Game/FPS/Blueprints/BlueprintsComponents/AC_MatchStateSystem.AC_MatchStateSystem_C"))
  ;[0 0 0] On BecomeViewTarget
  (Networking|CanExecuteCosmeticEvents
    (:True
      (EventDispatchers|BindEventtoOnPostRound _returnvalue_3 (delegate Custom|DestroyWidget))
      (EventDispatchers|BindEventtoOnPostMatch _returnvalue_3 (delegate Custom|DestroyWidget))
      (if (== PC (Game|GetPlayerController 0))
        (Utilities|FlowControl|Sequence
          (:then_0
            (Utilities|IsValid _returnvalue_2
              (:Is%20Valid
                (bind _returnvalue_4 (UserInterface|CreateWidget "/Game/FPS/UI/GameMode/SearchAndDestroy/WB_SpectatorWidget.WB_SpectatorWidget_C" _returnvalue_2))
                (bind _output_get (Variables|Default|SetWB_Spectator _returnvalue_4))
                (UserInterface|Viewport|AddtoViewport _output_get 0)
                (EventDispatchers|AssignCanRespawn _returnvalue_4 (delegate Custom|CanRespawn)))))
          (:then_1
            (Input|EnableInput PC)
            (Input|AddMappingContext (PlayerController|LocalPlayerSubsystems|GetEnhancedInputLocalPlayerSubsystem (Game|GetPlayerController 0)) "/Game/FPS/Inputs/IMC_SpectatorInputs.IMC_SpectatorInputs" 1 "(bIgnoreAllPressedKeysUntilRelease=True,bForceImmediately=False)")
            (Utilities|FlowControl|Delay 1.0)
            (Variables|/Script/Engine.SpringArmComponent|SetbEnableCameraLag (Variables|Default|GetSpringArm) true)))))))

(fn ConstructionScript)