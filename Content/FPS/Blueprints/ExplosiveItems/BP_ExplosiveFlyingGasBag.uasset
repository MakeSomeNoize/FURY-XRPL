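; Explosive gas bag physics prop that punctures, flies erratically as it vents, then explodes.
; Damage from AnyDamage or IDamage is checked against puncture and explode thresholds; a puncture starts a delayed loop adding random damage until detonation.
; Venting repeatedly applies randomized force and torque with attached burst FX.
; Detonation spawns FX, applies radial damage and impulse, notifies nearby ISpecialExplosive actors for chain reactions, then hides and destroys the actor.
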(event OnComponentHit(StaticMeshComponent)
  (params (HitComponent :type Primitive%20Component%20Object%20Reference) (OtherActor :type Actor%20Object%20Reference) (OtherComp :type Primitive%20Component%20Object%20Reference) (NormalImpulse :type Vector :default "0, 0, 0") (Hit :type Hit%20Result%20Structure%20%28by%20ref%29))
  ;[1 1 1] Hit Results
  (if (Variables|Default|GetPunctured?)
    _))

(event Custom|Kill
  ;[1 1 1] Wait for FX to fade then kill actor
  (Actor|DestroyActor))

(event Custom|Explode
  (bind _returnvalue (Math|Random|RandomFloatinRange 1.5e+02 3e+02))
  (bind _returnvalue_2 (Math|Random|RandomFloatinRange -3.6e+02 3.6e+02))
  (bind _self self)
  (bind _staticmeshcomponent (Variables|Debug|GetStaticMeshComponent))
  (bind _damage_radius (Variables|Default|GetDamage%20Radius))
  (bind _staticmeshcomponent_2 (Variables|Debug|GetStaticMeshComponent))
  (bind _staticmeshcomponent_3 (Variables|Debug|GetStaticMeshComponent))
  (bind _returnvalue_3 (Transformation|GetWorldLocation _staticmeshcomponent_2))
  (bind _returnvalue_4 (Transformation|GetWorldLocation _staticmeshcomponent))
  ;[1 1 1] Explode Event Triggered
  (if (not (Variables|Default|GetShrapnelCompleted))
    (if (Class|PrimitiveComponent|IsOverlappingComponent (Variables|Debug|GetStaticMeshComponent) (.HitComponent (Collision|BreakHitResult (stale OnComponentHit(StaticMeshComponent) Hit))))
      ;[1 1 1] Surface Explosion
      (Effects|SpawnEmitteratLocation "/Game/Environment/VFX/Explosion_GrenadeLauncher_1.Explosion_GrenadeLauncher_1" (.Location (Collision|BreakHitResult (stale OnComponentHit(StaticMeshComponent) Hit))) (Math|Conversions|RotationFromXVector (.ImpactNormal (Collision|BreakHitResult (stale OnComponentHit(StaticMeshComponent) Hit)))))
      ;[1 1 1] Spawn Decal (pending)
      (Rendering|Decal|SpawnDecalatLocation "/Game/FPS/Environment/Decals/Decals_Metal.Decals_Metal" "120.000000,120.000000,120.000000" (.ImpactPoint (Collision|BreakHitResult (stale OnComponentHit(StaticMeshComponent) Hit))) (Math|Conversions|RotationFromXVector (.ImpactNormal (Collision|BreakHitResult (stale OnComponentHit(StaticMeshComponent) Hit)))) 0.0)
      (else
        ;[1 1 1] Explosion Mid Air
        (Effects|SpawnEmitteratLocation "/Game/Environment/VFX/Explosion_GrenadeLauncher_1.Explosion_GrenadeLauncher_1" (Transformation|GetWorldLocation (Variables|Debug|GetStaticMeshComponent)) (Math|Rotator|MakeRotfromZ (* (Class|KismetMathLibrary|RandomUnitVectorinConeinRadians (Math|Vector|GetUnitDirection(Vector) (.ImpactNormal (Collision|BreakHitResult (stale OnComponentHit(StaticMeshComponent) Hit))) "0, 0, 0") (Variables|Default|GetExplosion%20Angle%20Variance%20VFX)) -1.0)))))
    (Audio|Components|Audio|Stop (Variables|Default|GetPunctureVenting_cue))
    ;[1 1 1] BOOMIFICATION Sound!
    (Audio|SpawnSoundatLocation "/Game/FPS/Sound/Explosions/Wav/SW_Explosion_03.SW_Explosion_03" (Transformation|GetWorldLocation (Variables|Debug|GetStaticMeshComponent)) "0, 0, 0" 0.75 (Class|GameplayStatics|GetGlobalTimeDilation) 0.0 0 0)
    (Utilities|FlowControl|Sequence
      (:then_0
        ;[1 1 1] Impulse and Damage
        (Game|Damage|ApplyRadialDamage 1.5e+02 _returnvalue_3 _damage_radius "/Game/FPS/Blueprints/Weapons/DamageTypes/DT_Explosion.DT_Explosion_C" (Utilities|Array|MakeArray _self) _self (stale Game|Damage|EventAnyDamage InstigatedBy) false "ECC_Visibility")
        (Physics|AddRadialImpulse (.HitComponent (Collision|BreakHitResult (stale OnComponentHit(StaticMeshComponent) Hit))) _returnvalue_3 5e+02 1e+06 "RIF_Constant" false)
        ;[1 1 1] Shrapnel Switch - keep it on... you know you want to.
        (if (not (Variables|Shrapnel|GetShrapnelActivated?))
          (Utilities|FlowControl|Sequence
            (:then_0
              ;[1 1 1] Tidy Up
              (Variables|Default|SetShrapnelCompleted true)
              (Physics|SetSimulatePhysics (Variables|Debug|GetStaticMeshComponent) false)
              (Collision|SetCollisionEnabled _staticmeshcomponent_3 "NoCollision")
              (Rendering|SetVisibility _staticmeshcomponent_3 false false)
              (Utilities|IsValid (stale EventIDamage _returnvalue_11)
                (:Is%20Valid
                  (Effects|Components|ParticleSystem|SetEmitterEnable (stale EventIDamage _returnvalue_11) "Fire" false)
                  (Effects|Components|ParticleSystem|SetEmitterEnable (stale EventIDamage _returnvalue_11) "Sparks_flow" false))))
            (:then_1
              (bind (_outhit _returnvalue_5) (Collision|LineTraceByChannel _returnvalue_4 (+ _returnvalue_4 "0, 0,-100.000000") "TraceTypeQuery1" false 0 "None"))
              (if _returnvalue_5
                (bind _returnvalue_6 (Rendering|Decal|SpawnDecalatLocation "/Game/FPS/Effects/Materials/Explosion/M_scorch.M_scorch" (Math|Vector|MakeVector _returnvalue _returnvalue _returnvalue) (.Location (Collision|BreakHitResult _outhit)) (Math|Rotator|MakeRotator _returnvalue_2 -9e+01 _returnvalue_2) 0.0))
                (Rendering|Components|Decal|SetFadeOut _returnvalue_6 1e+01 3.0 true)
                (Camera|PlayWorldCameraShake "/Game/FPS/Blueprints/CameraShake/CS_Explosion.CS_Explosion_C" (.Location (Collision|BreakHitResult _outhit)) (* 5e+02 2.0) (* 5e+02 3.0))
                ;[1 1 1] Wait for FX to fade then kill actor
                (Utilities|FlowControl|Delay 3.0)
                (CallFunction|Kill))))))
      (:then_1
        (bind _outactors (Collision|SphereOverlapActors _returnvalue_3 _damage_radius (Utilities|Array|MakeArray "ObjectTypeQuery4") 0 (Utilities|Array|MakeArray self)))
        (for _array_element _outactors
          (if (Utilities|DoesObjectImplementInterface _array_element "/Game/FPS/Blueprints/Interfaces/iSpecialExplosive.iSpecialExplosive_C")
            (Class|ISpecialExplosive|IDamage(Message) _array_element 1.5e+02)))))))

(event Custom|Punctured
  (bind _damagecounterduration (Variables|Default|GetDamageCounterDuration))
  (bind _punctureventing_cue (Variables|Default|GetPunctureVenting_cue))
  ;[1 1 1] Recieve puncture event
  (Audio|Components|Audio|Play _punctureventing_cue 0.0)
  (Variables|/Script/Engine.AudioComponent|SetPitchMultiplier _punctureventing_cue (Class|GameplayStatics|GetGlobalTimeDilation))
  ;[1 1 1] Apply damage over time
  (Variables|Default|SetDamage (+ (Variables|Default|GetDamage) (Math|Random|RandomFloatinRange 25.0 8e+01)) :!label _label)
  ;[1 1 1] Call explode when damage reached
  (if (>= (Variables|Default|GetDamage) (Variables|DamageThresholds|GetDamage%20to%20explode))
    (CallFunction|Explode)
    (else
      (Utilities|FlowControl|Delay (+ _damagecounterduration (- _damagecounterduration (Class|GameplayStatics|GetGlobalTimeDilation))))
      (goto _label))))

(event EventIDamage
  (params (Damage :type Float%20%28double-precision%29))
  (bind _returnvalue (Math|Random|RandomFloatinRange 1.5e+02 3e+02))
  (bind _returnvalue_2 (Math|Random|RandomFloatinRange -2e+02 2e+02))
  (bind _returnvalue_3 (Math|Random|RandomFloatinRange -2e+02 2e+02))
  (bind _returnvalue_4 (Math|Random|RandomFloatinRange -2e+02 2e+02))
  (bind _returnvalue_5 (Math|Random|RandomFloatinRange -3.6e+02 3.6e+02))
  (bind _self self)
  (bind _staticmeshcomponent (Variables|Debug|GetStaticMeshComponent))
  (bind _damage_radius (Variables|Default|GetDamage%20Radius))
  (bind _staticmeshcomponent_2 (Variables|Debug|GetStaticMeshComponent))
  (bind _staticmeshcomponent_3 (Variables|Debug|GetStaticMeshComponent))
  (bind _returnvalue_6 (Transformation|GetWorldLocation _staticmeshcomponent_2))
  (bind _returnvalue_7 (Transformation|GetWorldLocation _staticmeshcomponent))
  (bind _returnvalue_8 (Math|Vector|MakeVector _returnvalue_3 _returnvalue_4 _returnvalue_2))
  ;[1 1 1] Set Standard Damage
  (Variables|Default|SetDamage (+ (Variables|Default|GetDamage) Damage))
  ;[1 1 1] Damage Threshold Checks
  (if (>= (Variables|Default|GetDamage) (Variables|DamageThresholds|GetDamage%20to%20puncture))
    (if (not (Variables|Default|GetPunctured?))
      (Variables|Default|SetPunctured? true)
      (CallFunction|Punctured)
      (if (>= (Variables|Default|GetDamage) (Variables|DamageThresholds|GetDamage%20to%20explode))
        (Variables|Default|SetExploding true)
        ;[1 1 1] Explode Event Triggered
        (if (not (Variables|Default|GetShrapnelCompleted))
          (if (Class|PrimitiveComponent|IsOverlappingComponent (Variables|Debug|GetStaticMeshComponent) (.HitComponent (Collision|BreakHitResult (stale OnComponentHit(StaticMeshComponent) Hit))))
            ;[1 1 1] Surface Explosion
            (Effects|SpawnEmitteratLocation "/Game/Environment/VFX/Explosion_GrenadeLauncher_1.Explosion_GrenadeLauncher_1" (.Location (Collision|BreakHitResult (stale OnComponentHit(StaticMeshComponent) Hit))) (Math|Conversions|RotationFromXVector (.ImpactNormal (Collision|BreakHitResult (stale OnComponentHit(StaticMeshComponent) Hit)))))
            ;[1 1 1] Spawn Decal (pending)
            (Rendering|Decal|SpawnDecalatLocation "/Game/FPS/Environment/Decals/Decals_Metal.Decals_Metal" "120.000000,120.000000,120.000000" (.ImpactPoint (Collision|BreakHitResult (stale OnComponentHit(StaticMeshComponent) Hit))) (Math|Conversions|RotationFromXVector (.ImpactNormal (Collision|BreakHitResult (stale OnComponentHit(StaticMeshComponent) Hit)))) 0.0)
            (else
              ;[1 1 1] Explosion Mid Air
              (Effects|SpawnEmitteratLocation "/Game/Environment/VFX/Explosion_GrenadeLauncher_1.Explosion_GrenadeLauncher_1" (Transformation|GetWorldLocation (Variables|Debug|GetStaticMeshComponent)) (Math|Rotator|MakeRotfromZ (* (Class|KismetMathLibrary|RandomUnitVectorinConeinRadians (Math|Vector|GetUnitDirection(Vector) (.ImpactNormal (Collision|BreakHitResult (stale OnComponentHit(StaticMeshComponent) Hit))) "0, 0, 0") (Variables|Default|GetExplosion%20Angle%20Variance%20VFX)) -1.0)))))
          (Audio|Components|Audio|Stop (Variables|Default|GetPunctureVenting_cue))
          ;[1 1 1] BOOMIFICATION Sound!
          (Audio|SpawnSoundatLocation "/Game/FPS/Sound/Explosions/Wav/SW_Explosion_03.SW_Explosion_03" (Transformation|GetWorldLocation (Variables|Debug|GetStaticMeshComponent)) "0, 0, 0" 0.75 (Class|GameplayStatics|GetGlobalTimeDilation) 0.0 0 0)
          (Utilities|FlowControl|Sequence
            (:then_0
              ;[1 1 1] Impulse and Damage
              (Game|Damage|ApplyRadialDamage 1.5e+02 _returnvalue_6 _damage_radius "/Game/FPS/Blueprints/Weapons/DamageTypes/DT_Explosion.DT_Explosion_C" (Utilities|Array|MakeArray _self) _self (stale Game|Damage|EventAnyDamage InstigatedBy) false "ECC_Visibility")
              (Physics|AddRadialImpulse (.HitComponent (Collision|BreakHitResult (stale OnComponentHit(StaticMeshComponent) Hit))) _returnvalue_6 5e+02 1e+06 "RIF_Constant" false)
              ;[1 1 1] Shrapnel Switch - keep it on... you know you want to.
              (if (not (Variables|Shrapnel|GetShrapnelActivated?))
                (Utilities|FlowControl|Sequence
                  (:then_0
                    ;[1 1 1] Tidy Up
                    (Variables|Default|SetShrapnelCompleted true)
                    (Physics|SetSimulatePhysics (Variables|Debug|GetStaticMeshComponent) false)
                    (Collision|SetCollisionEnabled _staticmeshcomponent_3 "NoCollision")
                    (Rendering|SetVisibility _staticmeshcomponent_3 false false)
                    (Utilities|IsValid (stale _returnvalue_11)
                      (:Is%20Valid
                        (Effects|Components|ParticleSystem|SetEmitterEnable (stale _returnvalue_11) "Fire" false)
                        (Effects|Components|ParticleSystem|SetEmitterEnable (stale _returnvalue_11) "Sparks_flow" false))))
                  (:then_1
                    (bind (_outhit _returnvalue_9) (Collision|LineTraceByChannel _returnvalue_7 (+ _returnvalue_7 "0, 0,-100.000000") "TraceTypeQuery1" false 0 "None"))
                    (if _returnvalue_9
                      (bind _returnvalue_10 (Rendering|Decal|SpawnDecalatLocation "/Game/FPS/Effects/Materials/Explosion/M_scorch.M_scorch" (Math|Vector|MakeVector _returnvalue _returnvalue _returnvalue) (.Location (Collision|BreakHitResult _outhit)) (Math|Rotator|MakeRotator _returnvalue_5 -9e+01 _returnvalue_5) 0.0))
                      (Rendering|Components|Decal|SetFadeOut _returnvalue_10 1e+01 3.0 true)
                      (Camera|PlayWorldCameraShake "/Game/FPS/Blueprints/CameraShake/CS_Explosion.CS_Explosion_C" (.Location (Collision|BreakHitResult _outhit)) (* 5e+02 2.0) (* 5e+02 3.0))
                      ;[1 1 1] Wait for FX to fade then kill actor
                      (Utilities|FlowControl|Delay 3.0)
                      (CallFunction|Kill))))))
            (:then_1
              (bind _outactors (Collision|SphereOverlapActors _returnvalue_6 _damage_radius (Utilities|Array|MakeArray "ObjectTypeQuery4") 0 (Utilities|Array|MakeArray self)))
              (for _array_element _outactors
                (if (Utilities|DoesObjectImplementInterface _array_element "/Game/FPS/Blueprints/Interfaces/iSpecialExplosive.iSpecialExplosive_C")
                  (Class|ISpecialExplosive|IDamage(Message) _array_element 1.5e+02))))))
        (elif (not (Variables|Default|GetVenting))
          ;[1 1 1] Trail FX
          (bind _returnvalue_11 (Effects|SpawnEmitterAttached "/Game/Environment/VFX/Burst.Burst" (Variables|Default|GetArrow) "None" "0, 0, 0" (Math|Conversions|RotationFromXVector _returnvalue_8) "1.000000,1.000000,1.000000" "SnapToTarget" false))
          ;[1 1 1] Force and Torque
          (Variables|Default|SetVenting true)
          (Physics|AddForce (Variables|Debug|GetStaticMeshComponent) (* (* (Class|KismetMathLibrary|RandomUnitVectorinConeinRadians (Math|Rotator|GetRotationXVector (Math|Rotator|MakeRotfromZ (* (Class|KismetMathLibrary|RandomUnitVectorinConeinRadians (Math|Vector|GetUnitDirection(Vector) (.Location (Collision|BreakHitResult (stale OnComponentHit(StaticMeshComponent) Hit))) "0, 0, 0") (Variables|Default|GetAngleFX)) 1.0))) 25.0) (* (Physics|GetMass (Variables|Debug|GetStaticMeshComponent)) (Math|Random|RandomFloatinRange 8e+03 4.2e+04))) (Variables|Force|GetPropellant%20Force%20Multiplier)) "None" false :!label _label)
          (Class|PrimitiveComponent|AddTorqueinDegrees (Variables|Debug|GetStaticMeshComponent) _returnvalue_8 "None" true)
          (Utilities|FlowControl|Delay 0.05)
          (if (not (Variables|Default|GetShrapnelCompleted))
            (goto _label)))))))

(event Game|Damage|EventAnyDamage
  (params (Damage :type Float%20%28single-precision%29) (DamageType :type Damage%20Type%20Object%20Reference) (InstigatedBy :type Controller%20Object%20Reference) (DamageCauser :type Actor%20Object%20Reference))
  (bind _returnvalue (Math|Random|RandomFloatinRange 1.5e+02 3e+02))
  (bind _returnvalue_2 (Math|Random|RandomFloatinRange -2e+02 2e+02))
  (bind _returnvalue_3 (Math|Random|RandomFloatinRange -2e+02 2e+02))
  (bind _returnvalue_4 (Math|Random|RandomFloatinRange -2e+02 2e+02))
  (bind _returnvalue_5 (Math|Random|RandomFloatinRange -3.6e+02 3.6e+02))
  (bind _self self)
  (bind _staticmeshcomponent (Variables|Debug|GetStaticMeshComponent))
  (bind _damage_radius (Variables|Default|GetDamage%20Radius))
  (bind _staticmeshcomponent_2 (Variables|Debug|GetStaticMeshComponent))
  (bind _staticmeshcomponent_3 (Variables|Debug|GetStaticMeshComponent))
  (bind _returnvalue_6 (Transformation|GetWorldLocation _staticmeshcomponent_2))
  (bind _returnvalue_7 (Transformation|GetWorldLocation _staticmeshcomponent))
  (bind _returnvalue_8 (Math|Vector|MakeVector _returnvalue_3 _returnvalue_4 _returnvalue_2))
  ;[1 1 1] Set Standard Damage
  (Variables|Default|SetDamage (+ (Variables|Default|GetDamage) Damage))
  ;[1 1 1] Damage Threshold Checks
  (if (>= (Variables|Default|GetDamage) (Variables|DamageThresholds|GetDamage%20to%20puncture))
    (if (not (Variables|Default|GetPunctured?))
      (Variables|Default|SetPunctured? true)
      (CallFunction|Punctured)
      (if (>= (Variables|Default|GetDamage) (Variables|DamageThresholds|GetDamage%20to%20explode))
        (Variables|Default|SetExploding true)
        ;[1 1 1] Explode Event Triggered
        (if (not (Variables|Default|GetShrapnelCompleted))
          (if (Class|PrimitiveComponent|IsOverlappingComponent (Variables|Debug|GetStaticMeshComponent) (.HitComponent (Collision|BreakHitResult (stale OnComponentHit(StaticMeshComponent) Hit))))
            ;[1 1 1] Surface Explosion
            (Effects|SpawnEmitteratLocation "/Game/Environment/VFX/Explosion_GrenadeLauncher_1.Explosion_GrenadeLauncher_1" (.Location (Collision|BreakHitResult (stale OnComponentHit(StaticMeshComponent) Hit))) (Math|Conversions|RotationFromXVector (.ImpactNormal (Collision|BreakHitResult (stale OnComponentHit(StaticMeshComponent) Hit)))))
            ;[1 1 1] Spawn Decal (pending)
            (Rendering|Decal|SpawnDecalatLocation "/Game/FPS/Environment/Decals/Decals_Metal.Decals_Metal" "120.000000,120.000000,120.000000" (.ImpactPoint (Collision|BreakHitResult (stale OnComponentHit(StaticMeshComponent) Hit))) (Math|Conversions|RotationFromXVector (.ImpactNormal (Collision|BreakHitResult (stale OnComponentHit(StaticMeshComponent) Hit)))) 0.0)
            (else
              ;[1 1 1] Explosion Mid Air
              (Effects|SpawnEmitteratLocation "/Game/Environment/VFX/Explosion_GrenadeLauncher_1.Explosion_GrenadeLauncher_1" (Transformation|GetWorldLocation (Variables|Debug|GetStaticMeshComponent)) (Math|Rotator|MakeRotfromZ (* (Class|KismetMathLibrary|RandomUnitVectorinConeinRadians (Math|Vector|GetUnitDirection(Vector) (.ImpactNormal (Collision|BreakHitResult (stale OnComponentHit(StaticMeshComponent) Hit))) "0, 0, 0") (Variables|Default|GetExplosion%20Angle%20Variance%20VFX)) -1.0)))))
          (Audio|Components|Audio|Stop (Variables|Default|GetPunctureVenting_cue))
          ;[1 1 1] BOOMIFICATION Sound!
          (Audio|SpawnSoundatLocation "/Game/FPS/Sound/Explosions/Wav/SW_Explosion_03.SW_Explosion_03" (Transformation|GetWorldLocation (Variables|Debug|GetStaticMeshComponent)) "0, 0, 0" 0.75 (Class|GameplayStatics|GetGlobalTimeDilation) 0.0 0 0)
          (Utilities|FlowControl|Sequence
            (:then_0
              ;[1 1 1] Impulse and Damage
              (Game|Damage|ApplyRadialDamage 1.5e+02 _returnvalue_6 _damage_radius "/Game/FPS/Blueprints/Weapons/DamageTypes/DT_Explosion.DT_Explosion_C" (Utilities|Array|MakeArray _self) _self InstigatedBy false "ECC_Visibility")
              (Physics|AddRadialImpulse (.HitComponent (Collision|BreakHitResult (stale OnComponentHit(StaticMeshComponent) Hit))) _returnvalue_6 5e+02 1e+06 "RIF_Constant" false)
              ;[1 1 1] Shrapnel Switch - keep it on... you know you want to.
              (if (not (Variables|Shrapnel|GetShrapnelActivated?))
                (Utilities|FlowControl|Sequence
                  (:then_0
                    ;[1 1 1] Tidy Up
                    (Variables|Default|SetShrapnelCompleted true)
                    (Physics|SetSimulatePhysics (Variables|Debug|GetStaticMeshComponent) false)
                    (Collision|SetCollisionEnabled _staticmeshcomponent_3 "NoCollision")
                    (Rendering|SetVisibility _staticmeshcomponent_3 false false)
                    (Utilities|IsValid (stale _returnvalue_11)
                      (:Is%20Valid
                        (Effects|Components|ParticleSystem|SetEmitterEnable (stale _returnvalue_11) "Fire" false)
                        (Effects|Components|ParticleSystem|SetEmitterEnable (stale _returnvalue_11) "Sparks_flow" false))))
                  (:then_1
                    (bind (_outhit _returnvalue_9) (Collision|LineTraceByChannel _returnvalue_7 (+ _returnvalue_7 "0, 0,-100.000000") "TraceTypeQuery1" false 0 "None"))
                    (if _returnvalue_9
                      (bind _returnvalue_10 (Rendering|Decal|SpawnDecalatLocation "/Game/FPS/Effects/Materials/Explosion/M_scorch.M_scorch" (Math|Vector|MakeVector _returnvalue _returnvalue _returnvalue) (.Location (Collision|BreakHitResult _outhit)) (Math|Rotator|MakeRotator _returnvalue_5 -9e+01 _returnvalue_5) 0.0))
                      (Rendering|Components|Decal|SetFadeOut _returnvalue_10 1e+01 3.0 true)
                      (Camera|PlayWorldCameraShake "/Game/FPS/Blueprints/CameraShake/CS_Explosion.CS_Explosion_C" (.Location (Collision|BreakHitResult _outhit)) (* 5e+02 2.0) (* 5e+02 3.0))
                      ;[1 1 1] Wait for FX to fade then kill actor
                      (Utilities|FlowControl|Delay 3.0)
                      (CallFunction|Kill))))))
            (:then_1
              (bind _outactors (Collision|SphereOverlapActors _returnvalue_6 _damage_radius (Utilities|Array|MakeArray "ObjectTypeQuery4") 0 (Utilities|Array|MakeArray self)))
              (for _array_element _outactors
                (if (Utilities|DoesObjectImplementInterface _array_element "/Game/FPS/Blueprints/Interfaces/iSpecialExplosive.iSpecialExplosive_C")
                  (Class|ISpecialExplosive|IDamage(Message) _array_element 1.5e+02))))))
        (elif (not (Variables|Default|GetVenting))
          ;[1 1 1] Trail FX
          (bind _returnvalue_11 (Effects|SpawnEmitterAttached "/Game/Environment/VFX/Burst.Burst" (Variables|Default|GetArrow) "None" "0, 0, 0" (Math|Conversions|RotationFromXVector _returnvalue_8) "1.000000,1.000000,1.000000" "SnapToTarget" false))
          ;[1 1 1] Force and Torque
          (Variables|Default|SetVenting true)
          (Physics|AddForce (Variables|Debug|GetStaticMeshComponent) (* (* (Class|KismetMathLibrary|RandomUnitVectorinConeinRadians (Math|Rotator|GetRotationXVector (Math|Rotator|MakeRotfromZ (* (Class|KismetMathLibrary|RandomUnitVectorinConeinRadians (Math|Vector|GetUnitDirection(Vector) (.Location (Collision|BreakHitResult (stale OnComponentHit(StaticMeshComponent) Hit))) "0, 0, 0") (Variables|Default|GetAngleFX)) 1.0))) 25.0) (* (Physics|GetMass (Variables|Debug|GetStaticMeshComponent)) (Math|Random|RandomFloatinRange 8e+03 4.2e+04))) (Variables|Force|GetPropellant%20Force%20Multiplier)) "None" false :!label _label)
          (Class|PrimitiveComponent|AddTorqueinDegrees (Variables|Debug|GetStaticMeshComponent) _returnvalue_8 "None" true)
          (Utilities|FlowControl|Delay 0.05)
          (if (not (Variables|Default|GetShrapnelCompleted))
            (goto _label)))))))

(fn ConstructionScript
  (Variables|Actor|SetbCanBeDamaged false)
  (Variables|Default|SetDamage 0.0)
  (Collision|SetCollisionProfileName (Variables|Debug|GetStaticMeshComponent) "PhysicsActor" true :!class /Script/Engine.PrimitiveComponent))