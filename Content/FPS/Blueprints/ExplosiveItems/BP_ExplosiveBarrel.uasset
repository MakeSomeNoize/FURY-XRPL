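; Networked explosive barrel that explodes when its HealthComponent dies, or three seconds after a first non-lethal hit sets it burning.
; The explosion applies radial damage, messages overlapped physics bodies implementing ISpecialExplosive, and multicasts particles, sound and camera shake.
; Death wakes net dormancy, and the destroyed RepNotify swaps in a physics-simulated wreck with a random upward impulse, removing the health component and fire.
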(event Custom|PlayEffectCombustion
  (Networking|CanExecuteCosmeticEvents
    (:True
      (bind _returnvalue (Effects|SpawnEmitteratLocation "/Game/Environment/VFX/Particles/Barrel/P_Barrel_Fire.P_Barrel_Fire" (Transformation|GetActorLocation self) "0, 0, 0" "0.500000,0.500000,0.500000"))
      (Variables|Default|SetP_Combustion _returnvalue))))

(event Custom|Explode
  (params (Instigator :type Controller%20Object%20Reference))
  (bind _returnvalue (Transformation|GetActorLocation))
  (bind _returnvalue_2 (Transformation|GetActorLocation))
  (bind _self self)
  (bind _array (Utilities|Array|MakeArray _self))
  ;[0 0 0] Explode
  (Utilities|FlowControl|Sequence
    (:then_0
      (Game|Damage|ApplyRadialDamage 2e+02 (Math|Vector|MakeVector (.x _returnvalue) (.y _returnvalue) (+ (.z _returnvalue) 8e+01)) (Variables|Default|GetRadius) "/Game/FPS/Blueprints/Weapons/DamageTypes/DT_Explosion.DT_Explosion_C" _array _self Instigator false "ECC_Visibility")
      (CallFunction|MulticastPlayCosmeticEffects)
      (Actor|SetLifeSpan 15.0))
    (:then_1
      (bind _outactors (Collision|SphereOverlapActors (Math|Vector|MakeVector (.x _returnvalue_2) (.y _returnvalue_2) (+ (.z _returnvalue_2) 8e+01)) (Variables|Default|GetRadius) (Utilities|Array|MakeArray "ObjectTypeQuery4") 0 _array))
      (for _array_element _outactors
        (if (Utilities|DoesObjectImplementInterface _array_element "/Game/FPS/Blueprints/Interfaces/iSpecialExplosive.iSpecialExplosive_C")
          (Class|ISpecialExplosive|IDamage(Message) _array_element 1.5e+02))))))

(event Custom|Multicast_PlayCosmeticEffects
  (bind _self self)
  (bind _radius (Variables|Default|GetRadius))
  (bind _returnvalue (Transformation|GetActorLocation _self))
  ;[0 0 0] Play Cosmetic effects
  (Networking|CanExecuteCosmeticEvents
    (:True
      (Effects|SpawnEmitteratLocation "/Game/Environment/VFX/Explosion_GrenadeLauncher_1.Explosion_GrenadeLauncher_1" _returnvalue)
      (Audio|PlaySoundatLocation "/Game/FPS/Sound/Explosions/SC_Explosion_with_Metal_Debris.SC_Explosion_with_Metal_Debris" _returnvalue "0, 0, 0" 0.5 1.0 0.0 "/Game/FPS/Sound/AudioSettings/Attenuation/ATT_Weapon.ATT_Weapon" 0 0 0)
      (Camera|PlayWorldCameraShake "/Game/FPS/Blueprints/CameraShake/CS_Explosion.CS_Explosion_C" _returnvalue (* _radius 2.0) (* _radius 3.0)))))

(event Game|Damage|EventAnyDamage
  (params (Damage :type Float%20%28single-precision%29) (DamageType :type Damage%20Type%20Object%20Reference) (InstigatedBy :type Controller%20Object%20Reference) (DamageCauser :type Actor%20Object%20Reference))
  (bind _healthcomponent (Variables|Default|GetHealthComponent))
  ;[0 0 0] Any Damage
  (if (not (Variables|Default|GetbDestroyed))
    (Utilities|IsValid InstigatedBy
      (:Is%20Valid
        (Class|IPawnActions|ShowHitMarker(Message) (Pawn|GetControlledPawn InstigatedBy) false))
      (:Is%20Not%20Valid
        _))
    (Default|HandleDamage _healthcomponent Damage)
    (if (Default|IsDead _healthcomponent)
      (Variables|Default|SetCombustion false)
      (Networking|SetNetDormancy "DORM_Awake")
      (Variables|Default|SetbDestroyed true :!label _label)
      (Networking|ForceNetUpdate)
      (CallFunction|Explode InstigatedBy)
      (else
        (Utilities|FlowControl|DoOnce false
          (:Completed
            (CallFunction|PlayEffectCombustion)
            (Variables|Default|SetCombustion true)
            (Utilities|FlowControl|Delay 3.0)
            (if (Variables|Default|GetCombustion)
              (goto _label))))))))

(fn ConstructionScript)

(fn OnRepBDestroyed
  (bind _barreldestroyedmesh (Variables|Default|GetBarrelDestroyedMesh))
  (bind _barrelmesh (Variables|Default|GetBarrelMesh))
  (bind _p_combustion (Variables|Default|GetP_Combustion))
  (bind _healthcomponent (Variables|Default|GetHealthComponent))
  (Rendering|SetVisibility _barrelmesh false false)
  (Collision|SetCollisionEnabled _barrelmesh "NoCollision")
  (Rendering|SetVisibility _barreldestroyedmesh true false)
  (Physics|SetSimulatePhysics _barreldestroyedmesh true)
  (Physics|AddImpulse _barreldestroyedmesh (Math|Vector|MakeVector (Math|Random|RandomFloatinRange 0.0 2e+02) (Math|Random|RandomFloatinRange 0.0 2e+02) (Math|Random|RandomFloatinRange 3e+02 6.5e+02)) "None" true)
  (Utilities|IsValid _healthcomponent
    (:Is%20Valid
      (Components|DestroyComponent _healthcomponent))
    (:Is%20Not%20Valid
      _))
  (Utilities|IsValid _p_combustion
    (:Is%20Valid
      (Components|DestroyComponent _p_combustion))))