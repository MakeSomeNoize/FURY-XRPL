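; BP_SMG is the SMG weapon Blueprint, handling visibility of its first-person and third-person mesh, magazine and magazine ammo components.
; The Reloading event hides the magazine ammo for a second, using the first-person component only for a locally controlled, non-ThirdPerson view.
; HideorShowChildrens toggles the FPP and TPP mesh sets based on ThirdPerson, while HideorShowChildrensALL shows just the third-person set.
; The construction script only calls its parent.
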(event EventHideorShowChildrens
  (if (Variables|Default|GetThird%20Person)
    (Rendering|SetVisibility (Variables|Default|GetMeshTPP) true false)
    (Rendering|SetVisibility (Variables|Default|GetMeshFPP) false true)
    (else
      (Rendering|SetVisibility (Variables|Default|GetMeshTPP) false true)
      (Rendering|SetVisibility (Variables|Default|GetMagazine) true false))))

(event EventReloading
  (params (IsLocalyContolled :type Boolean))
  (if IsLocalyContolled
    (if (Variables|Default|GetThird%20Person)
      (Rendering|SetVisibility (Variables|Default|GetAmmo_In_MagazineTPP) false false :!label _label)
      (Utilities|FlowControl|Delay 1.0)
      (Rendering|SetVisibility (Variables|Default|GetAmmo_In_MagazineTPP) true false)
      (else
        (Rendering|SetVisibility (Variables|Default|GetAmmo_In_Magazine) false false)
        (Utilities|FlowControl|Delay 1.0)
        (Rendering|SetVisibility (Variables|Default|GetAmmo_In_Magazine) true false)))
    (else
      (goto _label))))

(event EventHideorShowChildrensALL
  (Rendering|SetVisibility (Variables|Default|GetMeshTPP) true false))

(fn ConstructionScript
  (|CallParentFunction))