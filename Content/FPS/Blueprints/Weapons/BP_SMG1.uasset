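; SMG weapon Blueprint, a child class that manages the visibility of its first- and third-person gun and magazine meshes.
; HideorShowChildrens switches mesh sets on the ThirdPerson flag, while HideorShowChildrensALL shows the third-person mesh and magazine.
; Reloading uses fixed Delays to swap the full magazine for the empty one, hide it, then restore the full one.
; Non-locally controlled players always take the third-person reload path.
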(event EventReloading
  (params (IsLocalyContolled :type Boolean))
  (if IsLocalyContolled
    (if (Variables|Default|GetThird%20Person)
      (Rendering|SetVisibility (Variables|Default|GetMagazineTPP) false false :!label _label)
      (Rendering|SetVisibility (Variables|Default|GetMagazineEmptyTPP) true false)
      (Utilities|FlowControl|Delay 0.95)
      (Rendering|SetVisibility (Variables|Default|GetMagazineEmptyTPP) false false)
      (Utilities|FlowControl|Delay 0.35)
      (Rendering|SetVisibility (Variables|Default|GetMagazineTPP) true false)
      (else
        (Rendering|SetVisibility (Variables|Default|GetMagazine) false false)
        (Rendering|SetVisibility (Variables|Default|GetMagazineEmpty) true false)
        (Utilities|FlowControl|Delay 0.95)
        (Rendering|SetVisibility (Variables|Default|GetMagazineEmpty) false false)
        (Utilities|FlowControl|Delay 0.35)
        (Rendering|SetVisibility (Variables|Default|GetMagazine) true false)))
    (else
      (goto _label))))

(event EventHideorShowChildrens
  (if (Variables|Default|GetThird%20Person)
    (Rendering|SetVisibility (Variables|Default|GetMeshTPP) true false)
    (Rendering|SetVisibility (Variables|Default|GetMeshFPP) false true)
    (else
      (Rendering|SetVisibility (Variables|Default|GetMeshTPP) false true)
      (Rendering|SetVisibility (Variables|Default|GetMeshFPP) true false))))

(event EventHideorShowChildrensALL
  (Rendering|SetVisibility (Variables|Default|GetMeshTPP) true false))

(fn ConstructionScript
  (|CallParentFunction))