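; Assault rifle weapon Blueprint that manages visibility of its first-person and third-person meshes, magazines and ammo.
; Reloading shows both magazines, then hides the first after a short delay, using third-person parts for non-local players or third-person view.
; Inspecting plays the first-person inspect animation with the primary magazine shown.
; Separate events set component visibility for the current perspective or reveal selected third-person parts.
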(event EventInspecting
  (Components|Animation|PlayAnimation (Variables|Default|GetMeshFPP) "/Game/FPS/Weapons/AssaultRifle/Heat_772_Rifle/Animations/Heat_772_Animations/AS_Weapon_Heat_772_WeaponInspect.AS_Weapon_Heat_772_WeaponInspect" false)
  (Rendering|SetVisibility (Variables|Default|GetAmmo_In_Magazine) true false)
  (Rendering|SetVisibility (Variables|Default|GetAmmo_In_Magazine2) false true))

(event EventHideorShowChildrens
  (if (Variables|Default|GetThird%20Person)
    (Rendering|SetVisibility (Variables|Default|GetMeshTPP) true false)
    (Rendering|SetVisibility (Variables|Default|GetMeshFPP) false true)
    (else
      (Rendering|SetVisibility (Variables|Default|GetMeshTPP) false true)
      (Rendering|SetVisibility (Variables|Default|GetMagazine) true false))))

(event EventHideorShowChildrensALL
  (Rendering|SetVisibility (Variables|Default|GetMeshTPP) true false))

(event EventReloading
  (params (IsLocalyContolled :type Boolean))
  (if IsLocalyContolled
    (if (Variables|Default|GetThird%20Person)
      (Rendering|SetVisibility (Variables|Default|GetAmmo_In_MagazineTPP) false false :!label _label)
      (Rendering|SetVisibility (Variables|Default|GetMagazineTPP) true false)
      (Utilities|FlowControl|Delay 0.85)
      (Rendering|SetVisibility (Variables|Default|GetAmmo_In_MagazineTPP) false false)
      (Rendering|SetVisibility (Variables|Default|GetMagazineTPP) false true)
      (else
        (Rendering|SetVisibility (Variables|Default|GetAmmo_In_Magazine) false false)
        (Rendering|SetVisibility (Variables|Default|GetMagazine) true true)
        (Utilities|FlowControl|Delay 1.0)
        (Rendering|SetVisibility (Variables|Default|GetAmmo_In_Magazine) false false)
        (Rendering|SetVisibility (Variables|Default|GetMagazine) false true)))
    (else
      (goto _label))))

(fn ConstructionScript
  (|CallParentFunction))