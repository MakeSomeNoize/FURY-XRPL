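; BP_Knife is the knife weapon Blueprint, which an interacting pawn can pick up.
; On Interact it sends the instigator pawn an OnPickupWeaponMessage with its own class and a fixed ammo count, then destroys itself.
; The remaining interaction functions are stubs returning empty, zero or false values, and construction only calls the parent script.
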(event EventInteract
  (params (InstigatorPawn :type Pawn%20Object%20Reference))
  (Class|IPawnActions|OnPickupWeapon(Message) InstigatorPawn "BP_Knife_C" 11)
  (Actor|DestroyActor))

(fn ConstructionScript
  (|CallParentFunction))

(fn GetDescription
  (return ""))

(fn GetIcon
  (return 0))

(fn GetInteractTime
  (return 0.0))

(fn TrytoInteract
  (return false))