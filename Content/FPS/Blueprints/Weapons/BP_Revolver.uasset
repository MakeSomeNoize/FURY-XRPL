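; BP_Revolver is a child weapon Blueprint for the revolver, managing which first-person and third-person parts are visible.
; The visibility events switch mesh, sight and frame components by the ThirdPerson flag, with an ALL variant that only reveals the third-person parts.
; On reload it briefly shows a quick loader on a fixed delay, choosing the third-person one for non-local players or third-person view.
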(event EventBeginPlay
  (|CallParentFunction))

(event EventHideorShowChildrensALL
  (Rendering|SetVisibility (Variables|Default|GetSightTPP) true false))

(event EventReloading
  (params (IsLocalyContolled :type Boolean))
  (if IsLocalyContolled
    (if (Variables|Default|GetThird%20Person)
      (Rendering|SetVisibility (Variables|Default|GetQuick_LoaderTPP) true false :!label _label)
      (Utilities|FlowControl|Delay 1.11)
      (Rendering|SetVisibility (Variables|Default|GetQuick_LoaderTPP) false false)
      (else
        (Rendering|SetVisibility (Variables|Default|GetQuick_Loader) true false)
        (Utilities|FlowControl|Delay 1.11)
        (Rendering|SetVisibility (Variables|Default|GetQuick_Loader) false false)))
    (else
      (goto _label))))

(event EventHideorShowChildrens
  (if (Variables|Default|GetThird%20Person)
    (Rendering|SetVisibility (Variables|Default|GetMeshTPP) true false)
    (Rendering|SetVisibility (Variables|Default|GetMeshFPP) false true)
    (else
      (Rendering|SetVisibility (Variables|Default|GetQuick_Loader) false false)
      (Rendering|SetVisibility (Variables|Default|GetSkeleton_Frame) true false))))

(fn ConstructionScript
  (|CallParentFunction))