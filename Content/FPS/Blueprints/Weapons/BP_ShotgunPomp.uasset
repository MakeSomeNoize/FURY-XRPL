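; BP_ShotgunPomp is a shotgun weapon actor that can be picked up through interaction.
; HideorShowChildrens uses ThirdPerson to switch between FPP and TPP meshes, ironsights and stock, though the first-person branch leaves MeshTPP visibility untouched.
; HideorShowChildrensALL shows the TPP parts without hiding the FPP ones.
; Interact passes its class and a fixed ammo count to the instigator pawn's pickup message, then destroys the actor.
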(event EventBeginPlay
  (|CallParentFunction) ; This node is disabled and will not be called.\nDrag off pins to build functionality.
)

(event EventInteract
  (params (InstigatorPawn :type Pawn%20Object%20Reference))
  (Class|IPawnActions|OnPickupWeapon(Message) InstigatorPawn "BP_ShotgunPomp_C" 11)
  (Actor|DestroyActor))

(event EventHideorShowChildrens
  (if (Variables|Default|GetThird%20Person)
    (Rendering|SetVisibility (Variables|Default|GetMeshTPP) true false)
    (Rendering|SetVisibility (Variables|Default|GetMeshFPP) false false)
    (else
      (Rendering|SetVisibility (Variables|Default|GetIronsight_frontTPP) false false)
      (Rendering|SetVisibility (Variables|Default|GetIronsight_RearFPP) true false))))

(event EventHideorShowChildrensALL
  (Rendering|SetVisibility (Variables|Default|GetMeshTPP) true false))

(fn ConstructionScript
  (|CallParentFunction))

(fn GetDescription
  (return ""))

(fn GetIcon
  (return 0))

(fn GetInteractTime
  (return 0.0))

(fn TrytoInteract
  (return false))