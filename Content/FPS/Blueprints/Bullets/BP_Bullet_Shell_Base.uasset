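; BP_Bullet_Shell_Base is a base actor for ejected bullet shell casings, with a configurable mesh, lifetime and sound.
; The construction script applies the shell mesh to the Case component.
; On BeginPlay it impulses the case along the owner's right vector or backward, depending on IsRightVector.
; It then plays a quiet shell sound after a short delay, if one is set, and destroys itself after DestroyTime.
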(event EventBeginPlay
  (bind _returnvalue (Components|GetOwner))
  (bind _shellsound (Variables|Default|GetShellSound))
  (if (Variables|Default|GetisRightVector)
    (Variables|Default|SetImpulse (* (Transformation|GetActorRightVector _returnvalue) 4.3e+02))
    (else
      (Variables|Default|SetImpulse (* (Transformation|GetActorForwardVector _returnvalue) -4.3e+02))))
  (Physics|AddImpulse (Variables|Default|GetCase) (Variables|Default|GetImpulse) "" false)
  (Utilities|FlowControl|Sequence
    (:then_0
      (Utilities|FlowControl|Delay (Variables|Default|GetDestroyTime))
      (Actor|DestroyActor))
    (:then_1
      (Utilities|FlowControl|Delay 0.4)
      (Utilities|IsValid _shellsound
        (:Is%20Valid
          (Audio|PlaySoundatLocation _shellsound (Transformation|GetActorLocation) "0, 0, 0" 0.05 1.0 0.0 0 0 0 0))))))

(fn ConstructionScript
  (Components|StaticMesh|SetStaticMesh (Variables|Default|GetCase) (Variables|Default|GetSMBulletShell)))