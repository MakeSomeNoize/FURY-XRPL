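; Behavior tree task that makes a living AI pawn interact with nearby bomb objectives in the Rush game mode.
; On execute it checks the pawn's health component, then loops the bomb references held by the Rush game state.
; Each valid bomb within range receives an AI interact call, then the task clears the interact blackboard key and finishes successfully.
; A dead pawn or failed game state cast leaves the task without a FinishExecute call.
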(event EventReceiveExecuteAI
  (params (OwnerController :type AI%20Controller%20Object%20Reference) (ControlledPawn :type Pawn%20Object%20Reference))
  ;[0 0 0] Interact with objective
  (if (not (Default|IsDead (Actor|GetComponentbyClass ControlledPawn "/Game/FPS/Blueprints/BlueprintsComponents/AC_Health.AC_Health_C")))
    (bind _asbp_rush_gs (Utilities|Casting|CastToBP_Rush_GS (Game|GetGameState)))
    (for _array_element (Variables|/Game/FPS/Blueprints/GameModes/Rush/BP_Rush_GS.BP_Rush_GS_C|GetBombRef _asbp_rush_gs)
      (Utilities|IsValid _array_element
        (:Is%20Valid
          (if (<= (Math|Vector|VectorLength (- (Transformation|GetActorLocation _array_element) (Transformation|GetActorLocation ControlledPawn))) 5e+02)
            (Default|AIBombInteract _array_element ControlledPawn)))))
    (Class|BTFunctionLibrary|SetBlackboardValueasBool (Variables|Default|GetInteractBombKey) false)
    (AI|BehaviorTree|FinishExecute true)))